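; Crafting NPC Blueprint that toggles a crafting UI when its Interaction event fires.
; Opening creates Tool_WidgetBlueprint_Hoon, passes this NPC to it through GetNpc, adds it to the viewport and shows the mouse cursor.
; Closing removes the widget and hides the cursor.
; A WidgetRemoveEnvent binding made at BeginPlay clears the OnOff flag, without touching the cursor; SelectAnswer is empty.
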(event Custom|Remove
  (Variables|Default|SetOnOff false))

(event Collision|EventActorBeginOverlap
  (params (OtherActor :type Actor%20Object%20Reference)))

(event EventTick
  (params (DeltaSeconds :type Float%20%28single-precision%29)))

(event EventInteraction
  (bind _returnvalue (Game|GetPlayerController 0))
  ;[1 1 1] 제작 UI On/Off
  (if (Variables|Default|GetOnOff)
    (Widget|RemovefromParent (stale _returnvalue_2))
    (Variables|/Script/Engine.PlayerController|SetbShowMouseCursor _returnvalue false)
    (Variables|Default|SetOnOff false)
    (else
      (bind _returnvalue_2 (UserInterface|CreateWidget "/Game/통합/UI/CraftUI/Tool_WidgetBlueprint_Hoon.Tool_WidgetBlueprint_Hoon_C"))
      (Default|GetNpc _returnvalue_2 self)
      (UserInterface|Viewport|AddtoViewport _returnvalue_2 0)
      (Variables|Default|SetOnOff true)
      (Variables|/Script/Engine.PlayerController|SetbShowMouseCursor _returnvalue true))))

(event EventSelectAnswer
  (params (Selection :type EN_InteractionType%20Enum :default "NewEnumerator0")))

(event EventBeginPlay
  (EventDispatchers|BindEventtoWidgetRemoveEnvent (delegate Custom|Remove)))

(fn ConstructionScript)