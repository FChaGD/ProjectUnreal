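; Enemy character Blueprint that switches between attack and run behavior trees according to its Enemy1 type, with walk speed taken from Enemy1.
; Seeing a pawn or being overlapped stops AI logic and writes blackboard state.
; Sighting the player handles four types, while player overlap handles only two.
; After starting a tree, a one-time distance check clears the seen and attacked flags if the player is far away.
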(event OnSeePawn(PawnSensing)
  (params (Pawn :type Pawn%20Object%20Reference))
  (bind _self self)
  (bind _enemy1 (Variables|Default|GetEnemy1))
  (bind _returnvalue (AI|GetAIController _self))
  (bind _returnvalue_2 (AI|GetBlackboard _returnvalue))
  (AI|Logic|StopLogic (Variables|/Script/AIModule.AIController|GetBrainComponent _returnvalue) "")
  (AI|Components|Blackboard|SetValueasBool _returnvalue_2 (Utilities|Name|MakeLiteralName "HasSeenPlayer") true)
  (AI|Components|Blackboard|SetValueasEnum _returnvalue_2 (Utilities|Name|MakeLiteralName "Type") (.type _enemy1))
  (Utilities|Casting|CastToBP_Player Pawn)
  (if (Utilities|Enum|Equal(Enum) (.type _enemy1) "NewEnumerator0")
    (AI|RunBehaviorTree _returnvalue "/Game/SeoK/Enemy/AI/BT_AttackEnemy.BT_AttackEnemy")
    (if (> (Transformation|GetDistanceTo (Game|GetPlayerCharacter 0)) 1e+03) :!label _label
      (CallFunction|ResetState))
    (elif (Utilities|Enum|Equal(Enum) (.type _enemy1) "NewEnumerator2")
      (AI|RunBehaviorTree _returnvalue "/Game/SeoK/Enemy/AI/BT_RunEnemy.BT_RunEnemy")
      (goto _label)
      (elif (Utilities|Enum|Equal(Enum) (.type _enemy1) "NewEnumerator1")
        (AI|RunBehaviorTree _returnvalue "/Game/SeoK/Enemy/AI/BT_AttackEnemy.BT_AttackEnemy")
        (if (> (Transformation|GetDistanceTo (Game|GetPlayerCharacter 0)) 1e+03) :!label _label_2
          (CallFunction|ResetState))
        (elif (Utilities|Enum|Equal(Enum) (.type _enemy1) "NewEnumerator3")
          (AI|RunBehaviorTree _returnvalue "/Game/SeoK/Enemy/AI/BT_RunEnemy.BT_RunEnemy")
          (goto _label_2))))))

(event EventBeginPlay
  (Variables|/Script/Engine.CharacterMovementComponent|SetMaxWalkSpeed (Variables|Character|GetCharacterMovement self) (.spd (Variables|Default|GetEnemy1))))

(event EventTick
  (params (DeltaSeconds :type Float%20%28single-precision%29)))

(event Collision|EventActorBeginOverlap
  (params (OtherActor :type Actor%20Object%20Reference))
  (bind _self self)
  (bind _enemy1 (Variables|Default|GetEnemy1))
  (bind _returnvalue (AI|GetAIController _self))
  (bind _returnvalue_2 (AI|GetBlackboard _returnvalue))
  (AI|Logic|StopLogic (Variables|/Script/AIModule.AIController|GetBrainComponent (AI|GetAIController self)) "")
  (AI|Components|Blackboard|SetValueasBool _returnvalue_2 (Utilities|Name|MakeLiteralName "IsAttacked") true)
  (AI|Components|Blackboard|SetValueasEnum _returnvalue_2 (Utilities|Name|MakeLiteralName "Type") (.type _enemy1))
  (bind _asbp_player (Utilities|Casting|CastToBP_Player OtherActor))
  (if (Utilities|Enum|Equal(Enum) (.type _enemy1) "NewEnumerator1")
    (AI|RunBehaviorTree _returnvalue "/Game/SeoK/Enemy/AI/BT_AttackEnemy.BT_AttackEnemy")
    (if (> (Transformation|GetDistanceTo (Game|GetPlayerCharacter 0)) 1e+03) :!label _label
      (CallFunction|ResetState))
    (elif (Utilities|Enum|Equal(Enum) (.type _enemy1) "NewEnumerator3")
      (AI|RunBehaviorTree _returnvalue "/Game/SeoK/Enemy/AI/BT_RunEnemy.BT_RunEnemy")
      (goto _label))))

(fn ConstructionScript)

(fn ResetState
  (bind _self self)
  (bind _returnvalue (AI|GetAIController _self))
  (bind _returnvalue_2 (AI|GetBlackboard _returnvalue))
  (AI|Components|Blackboard|SetValueasBool _returnvalue_2 (Utilities|Name|MakeLiteralName "HasSeenPlayer") false)
  (AI|Components|Blackboard|SetValueasBool _returnvalue_2 (Utilities|Name|MakeLiteralName "IsAttacked") false))