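; BP_FireBall is a player fireball projectile that deals area damage after touching an actor.
; Overlap slows it to a near halt and starts a looping one-second timer, which is never cleared.
; Each tick of that timer swaps the flight particles for an explosion and applies radial damage, sparing the player, with a debug print.
; ExplosionCount only limits how many overlaps can restart the timer, not the number of blasts.
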(event EventBeginPlay
  (bind _output_get (Variables|Default|SetExplosionCount 3)))

(event Collision|EventActorBeginOverlap
  (params (OtherActor :type Actor%20Object%20Reference))
  (Variables|/Script/Engine.ProjectileMovementComponent|SetMaxSpeed (Variables|Default|GetProjectileMovement) 0.001)
  (if (> (stale EventBeginPlay _output_get) 0)
    (Utilities|Time|SetTimerbyFunctionName 0 "Fire Ball Attack" 1.0 true)
    (Variables|Default|SetExplosionCount (- (stale EventBeginPlay _output_get) 1))))

(event EventTick
  (params (DeltaSeconds :type Float%20%28single-precision%29)))

(fn ConstructionScript)

(fn FireBallAttack
  (Components|Activation|Deactivate (Variables|Default|GetParticleSystem))
  (Components|Activation|Activate (Variables|Default|GetFireBallExplosion) false)
  (Game|Damage|ApplyRadialDamage 15.0 (Transformation|GetActorLocation) 3e+02 0 (Utilities|Array|MakeArray (Game|GetPlayerCharacter 0) (Game|Player|GetPlayerPawn 0)) self (Game|GetPlayerController 0) true "ECC_Visibility")
  (Development|PrintString "15 Damage"))