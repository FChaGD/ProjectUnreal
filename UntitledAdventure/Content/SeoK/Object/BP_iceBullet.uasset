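; BP_iceBullet is an ice projectile that arcs from a given player location to a target actor and damages it.
; Init stores both and starts a timeline, lerping toward the target's live location with a curve-driven height offset, so it homes without collision sweeps.
; When the timeline finishes, it applies fixed damage credited to player controller 0, swaps effect components and destroys itself after a short delay.
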(event Custom|init
  (params (Target :type BP%20Enemy%20AI%20Object%20Reference) (PlayerLocation :type Vector))
  (Variables|Default|SetTarget Target)
  (Variables|Default|SetPlayer%20Location PlayerLocation)
  (CallFunction|ChaseStart))

(event Custom|chase%20start
  (bind (_direction _새_트랙_0 _새_트랙_1) (Timeline|타임라인 Play)
    (:Update
      (Transformation|SetActorLocation (Math|Vector|MakeVector (.x (Math|Vector|Lerp(Vector) (Variables|Default|GetPlayer%20Location) (Transformation|GetActorLocation (Variables|Default|GetTarget)) _새_트랙_1)) (.y (Math|Vector|Lerp(Vector) (Variables|Default|GetPlayer%20Location) (Transformation|GetActorLocation (Variables|Default|GetTarget)) _새_트랙_1)) (+ (.z (Math|Vector|Lerp(Vector) (Variables|Default|GetPlayer%20Location) (Transformation|GetActorLocation (Variables|Default|GetTarget)) _새_트랙_1)) (* _새_트랙_0 1e+02))) false false))
    (:Finished
      (CallFunction|IceBulletAttack))))

(fn ConstructionScript)

(fn IceBulletAttack
  (Game|Damage|ApplyDamage (Variables|Default|GetTarget) 3e+01 (Game|GetPlayerController 0) self)
  (Components|Activation|Activate (Variables|Default|GetBulletHit) false)
  (Components|Activation|Deactivate (Variables|Default|GetP_ky_waterBallHit))
  (Utilities|Time|SetTimerbyFunctionName 0 "Destroy Self" 2.0))

(fn DestroySelf
  (Actor|DestroyActor))