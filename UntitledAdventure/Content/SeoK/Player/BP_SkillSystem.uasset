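; BP_SkillSystem is a player skill Blueprint that tracks which skills are unlocked and at what tier.
; A SkillUnlocks map keys skill row names to tier counts.
; AddSkill inserts a new skill at tier one or increments an existing one, with no cap, and always returns true.
; QuerySkill reports whether a skill is unlocked and its tier, returning zero when absent.
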(event EventBeginPlay)

(event EventTick
  (params (DeltaSeconds :type Float%20%28single-precision%29)))

(fn AddSkill
  (params (Row_Name :type String))
  (bind _skillunlocks (Variables|Default|GetSkillUnlocks))
  (bind (_value _returnvalue) (Utilities|Map|Find _skillunlocks Row_Name))
  (if _returnvalue
    (Utilities|Map|Add (Variables|Default|GetSkillUnlocks) Row_Name (+ _value 1))
    (return true)
    (else
      (Utilities|Map|Add (Variables|Default|GetSkillUnlocks) Row_Name 1)
      (return true))))

(fn QuerySkill
  (params (Row_Name :type String))
  (bind _skillunlocks (Variables|Default|GetSkillUnlocks))
  (bind (_value _returnvalue) (Utilities|Map|Find _skillunlocks Row_Name))
  (if _returnvalue
    (return true _value)
    (else
      (return false 0))))