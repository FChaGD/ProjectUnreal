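; UI controller component for NPC dialogue that shows and removes the script box and the choice menu.
; Both widgets are created on first use, reused afterwards, and given the Caster on each show.
; Typing_2 reveals the script one character at a time through a re-armed one-shot timer with random delays for an uneven typewriter rhythm.
; FinishTheTyping overwrites the displayed text with the given script to cut typing short.
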(event Custom|Show%20Script
  (params (Name :type String) (Script :type String) (Caster :type BP%20F%20Cha%20NPC%20Base%20Object%20Reference))
  ;[1 1 1] 스크립트 출력
  (Variables|Default|SetDisplayScrpit "")
  (|Typing_2 Name Script Caster))

(event Custom|Finish%20The%20Typing
  (params (Script :type String))
  ;[1 1 1] 스크립트 출력
  (Variables|Default|SetDisplayScrpit Script))

(event Custom|Show%20Select
  (params (Caster :type BP%20F%20Cha%20NPC%20Base%20Object%20Reference))
  ;[1 1 1] 선택지 출력
  (Utilities|IsValid (Variables|Default|GetNPCSelect)
    (:Is%20Valid
      _)
    (:Is%20Not%20Valid
      ;;[1 1 1] ui 생성
      (bind _returnvalue (UserInterface|CreateWidget "/Game/차경환의_작업실/Widget/BP_NPCSelect.BP_NPCSelect_C" (Game|GetPlayerController 0)))
      (bind _output_get (Variables|Default|SetNPCSelect _returnvalue))))
  (Default|SetCaster _output_get Caster)
  (UserInterface|Viewport|AddtoViewport _output_get 0))

(event Custom|Clean%20Select
  ;[1 1 1] 선택지 제거
  (Widget|RemovefromParent (Variables|Default|GetNPCSelect)))

(event Custom|Clean%20Scirpt
  ;[1 1 1] 스크립트 ui 제거
  (Widget|RemovefromParent (Variables|Default|GetScriptWidget)))

(event EventBeginPlay)

(event EventTick
  (params (DeltaSeconds :type Float%20%28single-precision%29)))

(event Custom|RepeatTyping
  ;[1 1 1] UISetting
  (bind _returnvalue (Utilities|Time|SetTimerbyEvent (EventDispatchers|CreateEvent :!event Custom|TypeWriting) (Math|Random|RandomFloatinRange 0.02 0.07)))
  (Variables|Default|SettypeWriterTimer _returnvalue))

(event Custom|TypeWriting
  (Utilities|FlowControl|Sequence
    (:then_0
      ;[1 1 1] 스크립트 분할
      (Variables|Default|SetDisplayScrpit (Utilities|String|GetSubstring (stale _scrpit) 0 (+ (Utilities|String|Len (Variables|Default|GetDisplayScrpit)) 1))))
    (:then_1
      ;[1 1 1] UI 스크립트 출력
      (Default|SetContent (Variables|Default|GetScriptWidget) (Variables|Default|GetDisplayScrpit)))
    (:then_2
      ;[1 1 1] looping
      (if (Utilities|Enum|Equal(Enum) (stale _scrpit) (Variables|Default|GetDisplayScrpit))
        ;[1 1 1] 타이핑 종료
        (Utilities|Time|ClearandInvalidateTimerbyHandle (Variables|Default|GettypeWriterTimer))
        (Variables|Default|SetIstyping? false)
        (return)
        (else
          (CallFunction|RepeatTyping))))))