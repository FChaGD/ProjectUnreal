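; Game instance that owns the game's save file and persists player state to a single save slot.
; On Init it creates a BP_SL_SaveGame object, then swaps in the stored one if the slot exists.
; SaveGame calls LoadDataFromLevel to capture the player character's transform into SaveInformation, hands that to the save object and writes the slot.
; Only the transform is captured from the level; the other fields get zero or default values.
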(event EventInit
  (bind _returnvalue (SaveGame|CreateSaveGameObject "/Game/차경환의_작업실/SaveAndLoad/BP_SL_SaveGame.BP_SL_SaveGame_C"))
  (Variables|Default|SetSaveFile _returnvalue)
  (bind _returnvalue_2 (SaveGame|DoesSaveGameExist "saveslot"))
  (if _returnvalue_2
    (bind _returnvalue_3 (SaveGame|LoadGamefromSlot "saveslot"))
    (bind _asbp_sl_save_game (Utilities|Casting|CastToBP_SL_SaveGame _returnvalue_3))
    (Variables|Default|SetSaveFile _asbp_sl_save_game)))

(event EventSaveGame
  ;[1 1 1] 데이터 저장
  (CallFunction|LoadDatafromLevel)
  (Default|SaveData (Variables|Default|GetSaveFile) (Variables|Default|GetSaveInformation))
  (SaveGame|SaveGametoSlot (Variables|Default|GetSaveFile) "saveslot"))

(event EventLoadDatafromLevel
  (Variables|Default|SetSaveInformation (Utilities|Struct|MakeST_SaveInformation 0.0 (Transformation|GetActorTransform (Game|GetPlayerCharacter 0)) 0 0 0 0)))