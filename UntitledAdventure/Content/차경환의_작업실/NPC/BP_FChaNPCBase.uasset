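; Base NPC Blueprint that runs player-triggered dialogue with an opening script, an answer selection and a farewell script.
; Interaction switches on CurrentInteraction, stepping indexed script lines through the game mode's BPC_UIController, or finishing the current line early if still typing.
; The opening leads to the selection UI; choosing End plays the farewell, then resets indices and restores game-only input.
; InteractingEndSequnce is an empty event called during the flow.
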(event Custom|Interacting%20End%20Sequnce)

(event EventBeginPlay)

(event Collision|EventActorBeginOverlap
  (params (OtherActor :type Actor%20Object%20Reference)))

(event EventTick
  (params (DeltaSeconds :type Float%20%28single-precision%29)))

(event EventInteraction
  (bind _returnvalue (Game|GetPlayerController 0))
  (bind _returnvalue_2 (Game|GetPlayerController 0))
  (Class|ControllerInterface|ControllerHoldSet(Message) (Game|GetPlayerController 0) false)
  (switch Utilities|FlowControl|Switch|SwitchonEN_InteractionType (Variables|Default|GetCurrentInteraction)
    (:NewEnumerator0
      ;[1 1 1] 첫 상호작용 과정
      (|첫조우 (Variables|Default|GetFirstScript) :!label _label)
      (Default|CleanScirpt (Variables|Default|GetUI%20Controller))
      (Default|ShowSelect (Variables|Default|GetUI%20Controller) self)
      (Variables|Default|SetCurrentInteraction "NewEnumerator3"))
    (:NewEnumerator2
      ;[1 1 1] 대화 종료 과정
      (|대화종료 (Variables|Default|GetEndScript))
      (Variables|Default|SetFirstScript (Utilities|Struct|MakeBP_ScriptStructure -1 (.name (Variables|Default|GetFirstScript)) (.script (Variables|Default|GetFirstScript)) (.nextscript (Variables|Default|GetFirstScript))))
      (Variables|Default|SetEndScript (Utilities|Struct|MakeBP_ScriptStructure -1 (.name (Variables|Default|GetEndScript)) (.script (Variables|Default|GetEndScript)) (.nextscript (Variables|Default|GetEndScript))))
      (Default|CleanScirpt (Variables|Default|GetUI%20Controller))
      (Variables|Default|SetCurrentInteraction "NewEnumerator3")
      (Input|SetInputModeGameOnly _returnvalue_2 false)
      (Variables|/Script/Engine.PlayerController|SetbShowMouseCursor _returnvalue_2 false)
      (Class|ControllerInterface|ControllerHoldSet(Message) (Game|GetPlayerController 0) true))
    (:NewEnumerator3
      (Variables|Default|SetUI%20Controller (Actor|GetComponentbyClass (Game|GetGameMode) "/Game/차경환의_작업실/BPC_UIController.BPC_UIController_C"))
      (Input|SetInputModeGameandUI _returnvalue 0 "DoNotLock" true false)
      (Variables|/Script/Engine.PlayerController|SetbShowMouseCursor _returnvalue true)
      (Variables|Default|SetCurrentInteraction "NewEnumerator0")
      (goto _label)))
  (CallFunction|InteractingEndSequnce))

(event EventSelectAnswer
  (params (Selection :type EN_InteractionType%20Enum :default "NewEnumerator0"))
  (bind _returnvalue (Game|GetPlayerController 0))
  (switch Utilities|FlowControl|Switch|SwitchonEN_InteractionType Selection
    (:NewEnumerator2
      ;[1 1 1] 대화 종료 과정
      (Default|CleanSelect (Variables|Default|GetUI%20Controller))
      (Variables|Default|SetCurrentInteraction "NewEnumerator2")
      (|대화종료 (Variables|Default|GetEndScript))
      (Variables|Default|SetFirstScript (Utilities|Struct|MakeBP_ScriptStructure -1 (.name (Variables|Default|GetFirstScript)) (.script (Variables|Default|GetFirstScript)) (.nextscript (Variables|Default|GetFirstScript))))
      (Variables|Default|SetEndScript (Utilities|Struct|MakeBP_ScriptStructure -1 (.name (Variables|Default|GetEndScript)) (.script (Variables|Default|GetEndScript)) (.nextscript (Variables|Default|GetEndScript))))
      (Default|CleanScirpt (Variables|Default|GetUI%20Controller))
      (Variables|Default|SetCurrentInteraction "NewEnumerator3")
      (Input|SetInputModeGameOnly _returnvalue false)
      (Variables|/Script/Engine.PlayerController|SetbShowMouseCursor _returnvalue false)
      (Class|ControllerInterface|ControllerHoldSet(Message) (Game|GetPlayerController 0) true)
      (CallFunction|InteractingEndSequnce))))

(fn ConstructionScript)