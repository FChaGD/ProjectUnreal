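; Base NPC character that runs data-table-driven interactions: first meeting, talk, choices, speech bubbles and ending.
; Interaction switches on the current type, and FindLinkTableRow picks a script ID by NPC, progress range and lowest priority value.
; ScriptGenerate and GenerateBubble step through linked lines, finishing typing early and setting the next type, while SelectList feeds choices to UIController.
; Interaction also toggles player control and cursor; the end-sequence lookup matches rows but runs no actions.
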(event Custom|Interacting%20End%20Sequnce
  (params (InteractionId :type Integer))
  (bind _outrownames (DataTable|GetDataTableRowNames "/Game/통합/Table/BP_DT_EndSequence.BP_DT_EndSequence"))
  (for _array_element _outrownames
    (bind _returnvalue (Utilities|GetDataTableRow "/Game/통합/Table/BP_DT_EndSequence.BP_DT_EndSequence" _array_element)
      (:then
        (if (== InteractionId (.InteractionId (Utilities|Struct|BreakTS_EndSequence _returnvalue)))
          (switch Utilities|FlowControl|Switch|SwitchonEN_EndSequence (.EndSequence (Utilities|Struct|BreakTS_EndSequence _returnvalue))))))))

(event Custom|EndInteraction
  (bind _returnvalue (Game|GetPlayerController 0))
  ;[1 1 1] 상호작용 종료
  (Default|CleanScirpt (Variables|Default|GetUI%20Controller))
  (Variables|Default|SetCurrentInteraction "NewEnumerator3")
  (Input|SetInputModeGameOnly _returnvalue false)
  (Variables|/Script/Engine.PlayerController|SetbShowMouseCursor _returnvalue false)
  (Class|BPATIControllerInterface|ControllerHoldSet(Message) (Game|GetPlayerController 0) true))

(event Collision|EventActorBeginOverlap
  (params (OtherActor :type Actor%20Object%20Reference)))

(event EventTick
  (params (DeltaSeconds :type Float%20%28single-precision%29)))

(event EventInteraction
  (bind _returnvalue (Game|GetPlayerController 0))
  (bind _returnvalue_2 (Game|GetPlayerController 0))
  (if (and (Utilities|Enum|Equal(Enum) (Variables|Default|GetCurrentInteraction) "NewEnumerator3") (Utilities|Enum|Equal(Enum) "NewEnumerator6" (Variables|Default|GetDefaultInteraction)))
    _
    (elif (and (Utilities|Enum|NotEqual(Enum) (Variables|Default|GetCurrentInteraction) "NewEnumerator3") (Utilities|Enum|Equal(Enum) "NewEnumerator6" (Variables|Default|GetDefaultInteraction)))
      ;[1 1 1] 말풍선 상호작용 관련 inputmode & mouse cursor
      (Class|BPATIControllerInterface|ControllerHoldSet(Message) _returnvalue false)
      (Input|SetInputModeGameandUI _returnvalue 0 "DoNotLock" true false)
      (Variables|/Script/Engine.PlayerController|SetbShowMouseCursor _returnvalue true)
      (else
        (Class|BPATIControllerInterface|ControllerHoldSet(Message) (Game|GetPlayerController 0) false))))
  (switch Utilities|FlowControl|Switch|SwitchonEN_InteractionType (Variables|Default|GetCurrentInteraction) :!label _label
    (:NewEnumerator0
      ;[1 1 1] 첫 상호작용 과정
      (Variables|Default|SetCurrentInteraction "NewEnumerator0")
      (if (Variables|Default|GetIsScriptOver)
        _
        (else
          (bind _interactionidtarget (CallFunction|FindLinkTableRow "NewEnumerator0"))
          (Variables|Default|SetIsScriptOver true)))
      (bind _countinue (CallFunction|ScriptGenerate _interactionidtarget))
      (if _countinue
        (CallFunction|InteractingEndSequnce)))
    (:NewEnumerator1
      ;[1 1 1] 대화
      (Default|CleanSelect (Variables|Default|GetUI%20Controller))
      (Variables|Default|SetCurrentInteraction "NewEnumerator1")
      (if (Variables|Default|GetIsScriptOver)
        _
        (else
          (bind _interactionidtarget_2 (CallFunction|FindLinkTableRow "NewEnumerator1"))
          (Variables|Default|SetIsScriptOver true)))
      (bind (_endsequence _countinue_2) (CallFunction|ScriptGenerate _interactionidtarget_2))
      (if _countinue_2
        (CallFunction|InteractingEndSequnce _endsequence)))
    (:NewEnumerator2
      ;[1 1 1] 대화 종료 과정
      (if (Variables|Default|GetIsScriptOver)
        _
        (else
          (bind _interactionidtarget_3 (CallFunction|FindLinkTableRow "NewEnumerator2"))
          (Variables|Default|SetIsScriptOver true)))
      (bind (_endsequence_2 _countinue_3) (CallFunction|ScriptGenerate _interactionidtarget_3))
      (if _countinue_3
        (CallFunction|InteractingEndSequnce _endsequence_2)))
    (:NewEnumerator4
      (if (Variables|/Game/통합/Component/BPC_UIController.BPC_UIController_C|GetIstyping? (Variables|Default|GetUI%20Controller))
        ;[1 1 1] 선택지 전 스크립트 출력 예외처리
        (bind _returnvalue_3 (Utilities|GetDataTableRow (Variables|Default|GetScriptTable) (Utilities|String|StringToName (Utilities|String|ToString(Integer) (Variables|Default|GetPreScriptId))))
          (:then
            (Default|FinishtheTyping (Variables|Default|GetUI%20Controller) (.Script (Utilities|Struct|BreakTS_Script _returnvalue_3)))))
        (else
          ;[1 1 1] 선택지 상호작용
          (Default|CleanScirpt (Variables|Default|GetUI%20Controller))
          (bind _interactionidtarget_4 (CallFunction|FindLinkTableRow "NewEnumerator4"))
          (bind _selectlist (CallFunction|SelectList _interactionidtarget_4))
          (Default|ShowSelect (Variables|Default|GetUI%20Controller) self _selectlist)
          (Variables|Default|SetScriptId 0)
          (CallFunction|InteractingEndSequnce (Variables|Default|GetPreScriptId))
          (Variables|Default|SetPreScriptId 0))))
    (:NewEnumerator6
      ;[1 1 1] 상호작용
      (Variables|Default|SetCurrentInteraction "NewEnumerator6")
      (if (Variables|Default|GetIsScriptOver)
        _
        (else
          (bind _interactionidtarget_5 (CallFunction|FindLinkTableRow "NewEnumerator6"))
          (Variables|Default|SetIsScriptOver true)))
      (bind _endsequence_3 (CallFunction|GenerateBubble _interactionidtarget_5))
      (CallFunction|InteractingEndSequnce _endsequence_3))
    (:NewEnumerator3
      (if (== (Variables|Default|GetScriptId) -1)
        (Variables|Default|SetPreScriptId 0)
        (Variables|Default|SetScriptId 0)
        (CallFunction|EndInteraction)
        (else
          ;[1 1 1] 대화 종류가 아무것도 없을 경우
          (Variables|Default|SetUI%20Controller (Actor|GetComponentbyClass (Game|GetGameMode) "/Game/통합/Component/BPC_UIController.BPC_UIController_C"))
          (bind _output_get (Variables|Default|SetCurrentInteraction (Variables|Default|GetDefaultInteraction)))
          (if (Utilities|Enum|Equal(Enum) _output_get "NewEnumerator6")
            (goto _label)
            (else
              (Input|SetInputModeGameandUI _returnvalue_2 0 "DoNotLock" true false)
              (Variables|/Script/Engine.PlayerController|SetbShowMouseCursor _returnvalue_2 true)
              (goto _label))))))))

(event EventSelectAnswer
  (params (Selection :type EN_InteractionType%20Enum :default "NewEnumerator0"))
  (Class|BPATIControllerInterface|IsSelecting(Message) (Game|GetPlayerController 0) false)
  (switch Utilities|FlowControl|Switch|SwitchonEN_InteractionType Selection
    (:NewEnumerator0
      ;[1 1 1] 첫 상호작용 과정
      (Variables|Default|SetCurrentInteraction "NewEnumerator0")
      (if (Variables|Default|GetIsScriptOver)
        _
        (else
          (bind _interactionidtarget (CallFunction|FindLinkTableRow "NewEnumerator0"))
          (Variables|Default|SetIsScriptOver true)))
      (bind _countinue (CallFunction|ScriptGenerate _interactionidtarget))
      (if _countinue
        (CallFunction|InteractingEndSequnce)))
    (:NewEnumerator1
      ;[1 1 1] 대화
      (Default|CleanSelect (Variables|Default|GetUI%20Controller))
      (Variables|Default|SetCurrentInteraction "NewEnumerator1")
      (if (Variables|Default|GetIsScriptOver)
        _
        (else
          (bind _interactionidtarget_2 (CallFunction|FindLinkTableRow "NewEnumerator1"))
          (Variables|Default|SetIsScriptOver true)))
      (bind (_endsequence _countinue_2) (CallFunction|ScriptGenerate _interactionidtarget_2))
      (if _countinue_2
        (CallFunction|InteractingEndSequnce _endsequence)))
    (:NewEnumerator2
      ;[1 1 1] 대화 종료 과정
      (Default|CleanSelect (Variables|Default|GetUI%20Controller))
      (Variables|Default|SetCurrentInteraction "NewEnumerator2")
      (if (Variables|Default|GetIsScriptOver)
        _
        (else
          (bind _interactionidtarget_3 (CallFunction|FindLinkTableRow "NewEnumerator2"))
          (Variables|Default|SetIsScriptOver true)))
      (bind (_endsequence_2 _countinue_3) (CallFunction|ScriptGenerate _interactionidtarget_3))
      (if _countinue_3
        (CallFunction|InteractingEndSequnce _endsequence_2)))
    (:NewEnumerator4
      (if (Variables|/Game/통합/Component/BPC_UIController.BPC_UIController_C|GetIstyping? (Variables|Default|GetUI%20Controller))
        ;[1 1 1] 선택지 전 스크립트 출력 예외처리
        (bind _returnvalue (Utilities|GetDataTableRow (Variables|Default|GetScriptTable) (Utilities|String|StringToName (Utilities|String|ToString(Integer) (Variables|Default|GetPreScriptId))))
          (:then
            (Default|FinishtheTyping (Variables|Default|GetUI%20Controller) (.Script (Utilities|Struct|BreakTS_Script _returnvalue)))))
        (else
          ;[1 1 1] 선택지 상호작용
          (Default|CleanScirpt (Variables|Default|GetUI%20Controller))
          (bind _interactionidtarget_4 (CallFunction|FindLinkTableRow "NewEnumerator4"))
          (bind _selectlist (CallFunction|SelectList _interactionidtarget_4))
          (Default|ShowSelect (Variables|Default|GetUI%20Controller) self _selectlist)
          (Variables|Default|SetScriptId 0)
          (CallFunction|InteractingEndSequnce (Variables|Default|GetPreScriptId))
          (Variables|Default|SetPreScriptId 0))))
    (:NewEnumerator6
      ;[1 1 1] 상호작용
      (Variables|Default|SetCurrentInteraction "NewEnumerator6")
      (if (Variables|Default|GetIsScriptOver)
        _
        (else
          (bind _interactionidtarget_5 (CallFunction|FindLinkTableRow "NewEnumerator6"))
          (Variables|Default|SetIsScriptOver true)))
      (bind _endsequence_3 (CallFunction|GenerateBubble _interactionidtarget_5))
      (CallFunction|InteractingEndSequnce _endsequence_3))))

(fn ConstructionScript)

(fn ScriptGenerate
  (params (ScriptIdTarget :type Integer))
  ;[1 1 1] 기존 Id가 있는지 확인
  (if (== (Variables|Default|GetScriptId) 0)
    (bind _output_get (Variables|Default|SetScriptId ScriptIdTarget))
    (bind _returnvalue (Utilities|GetDataTableRow (Variables|Default|GetScriptTable) (Utilities|String|StringToName (Utilities|String|ToString(Integer) _output_get)) :!label _label)
      (:then
        _))
    (else
      ;[1 1 1] 상호작용이 끝났는지 확인
      (if (== (Variables|Default|GetScriptId) -1)
        _
        (else
          (goto _label)))))
  ;[1 1 1] UI가 타이핑 중인지 확인
  (if (Variables|/Game/통합/Component/BPC_UIController.BPC_UIController_C|GetIstyping? (Variables|Default|GetUI%20Controller))
    ;[1 1 1] 조기 타이핑 종료
    (bind _returnvalue_2 (Utilities|GetDataTableRow (Variables|Default|GetScriptTable) (Utilities|String|StringToName (Utilities|String|ToString(Integer) (Variables|Default|GetPreScriptId))))
      (:then
        (Default|FinishtheTyping (Variables|Default|GetUI%20Controller) (.Script (Utilities|Struct|BreakTS_Script _returnvalue_2)))
        (return (Variables|Default|GetPreScriptId) false)))
    (else
      ;[1 1 1] 상호작용이 끝났는지 확인
      (if (== (Variables|Default|GetScriptId) -1)
        ;[1 1 1] 다음 상호작용이 없으면 0으로 초기화
        (Variables|Default|SetScriptId 0)
        (Variables|Default|SetIsScriptOver false)
        (if (Utilities|Enum|Equal(Enum) (Variables|Default|GetCurrentInteraction) "NewEnumerator3")
          ;[1 1 1] 현재 상호작용이 None이면 상호작용, 아니면 endInteraction
          (CallFunction|Interaction)
          (Variables|Default|SetIsScriptOver false)
          (return (Variables|Default|GetPreScriptId) false)
          (else
            (CallFunction|EndInteraction)
            (Variables|Default|SetIsScriptOver false)
            (return (Variables|Default|GetPreScriptId) false)))
        (else
          ;[1 1 1] 대사 타이핑
          (Default|ShowScript (Variables|Default|GetUI%20Controller) (.Name (Utilities|Struct|BreakTS_Script _returnvalue)) (.Script (Utilities|Struct|BreakTS_Script _returnvalue)) self)
          (bind _returnvalue_3 (Utilities|GetDataTableRow "/Game/통합/Table/BP_DT_NextInteraction.BP_DT_NextInteraction" (Utilities|String|StringToName (Utilities|String|ToString(Integer) (Variables|Default|GetScriptId))))
            (:then
              (Variables|Default|SetCurrentInteraction (Utilities|Struct|BreakTS_NextInteraction _returnvalue_3))
              ;[1 1 1] 다음 스크립트가 있는지 확인
              (if (== 0 (.NextId (Utilities|Struct|BreakTS_Script _returnvalue)))
                ;[1 1 1] 다음 스크립트가 없으면 -1
                (Variables|Default|SetPreScriptId (Variables|Default|GetScriptId))
                (Variables|Default|SetScriptId -1)
                (Variables|Default|SetIsScriptOver false)
                (return (Variables|Default|GetPreScriptId) true)
                (else
                  ;[1 1 1] 다음 스크립트가 있을 경우
                  (Variables|Default|SetPreScriptId (Variables|Default|GetScriptId))
                  (Variables|Default|SetScriptId (.NextId (Utilities|Struct|BreakTS_Script _returnvalue)))
                  (return (Variables|Default|GetPreScriptId) true))))))))))

(fn FindLinkTableRow
  (params (TargetInteractionType :type EN_InteractionType%20Enum :default "NewEnumerator0"))
  (bind _currentprogress (Variables|Default|GetCurrentProgress))
  (bind _outrownames (DataTable|GetDataTableRowNames (Variables|Default|GetScriptLinkTable)))
  (for _array_element _outrownames
    (bind _returnvalue (Utilities|GetDataTableRow (Variables|Default|GetScriptLinkTable) _array_element)
      (:then
        ;[1 1 1] NPCId Check && Progress Check && TargetInteractionType Check
        (if (== (Variables|Default|GetNPC%20Num) (.NPCId (Utilities|Struct|BreakTS_InteractionLink _returnvalue)))
          (if (and (>= _currentprogress (.ProgressStart (Utilities|Struct|BreakTS_InteractionLink _returnvalue))) (< _currentprogress (.ProgressEnd (Utilities|Struct|BreakTS_InteractionLink _returnvalue))))
            (if (Utilities|Enum|Equal(Enum) TargetInteractionType (.InteractionType (Utilities|Struct|BreakTS_InteractionLink _returnvalue)))
              ;[1 1 1] Id와 priority 저장
              (Utilities|Array|Add (LocalVariables|GetInteractionIdList) (.InteractionId (Utilities|Struct|BreakTS_InteractionLink _returnvalue)))
              (Utilities|Array|Add (LocalVariables|GetPriorityList) (.Priority (Utilities|Struct|BreakTS_InteractionLink _returnvalue)))))))))
  ;[1 1 1] 같은 Interactiontype이 여러개 있는가?
  (if (>= (Utilities|Array|Length (LocalVariables|GetInteractionIdList)) 2)
    ;[1 1 1] 여러개라면 Priority로 결정
    (for (_array_element_2 _array_index) (LocalVariables|GetPriorityList)
      (if (< _array_element_2 (LocalVariables|GetMinChecker))
        (LocalVariables|SetMinChecker _array_element_2)
        (LocalVariables|SetMinIndex _array_index)))
    (bind _output_get (Variables|Default|SetInteractionIdTarget (Utilities|Array|Get(acopy) (LocalVariables|GetInteractionIdList) (LocalVariables|GetMinIndex))))
    (return _output_get)
    (else
      ;[1 1 1] 한개만 있을 경우
      (bind _output_get_2 (Variables|Default|SetInteractionIdTarget (Utilities|Array|Get(acopy) (LocalVariables|GetInteractionIdList))))
      (return _output_get_2))))

(fn SelectList
  (params (SelectId :type Integer))
  ;[1 1 1] Id가 맞는 데이터 찾기
  (bind _returnvalue (Class|DataTableFunctionLibrary|GetDataTableColumnasString "/Game/통합/Table/BP_DT_SelectTable.BP_DT_SelectTable" "InteractionId"))
  (for (_array_element _array_index) _returnvalue
    (if (Utilities|Enum|Equal(Enum) (Utilities|String|ToString(Integer) SelectId) _array_element)
      (Utilities|Array|Add (LocalVariables|GetSelectCollect) _array_index)))
  ;[1 1 1] 찾은 열을 리스트로 만들어서 제출
  (for _array_element_2 (LocalVariables|GetSelectCollect)
    (bind _returnvalue_2 (Class|DataTableFunctionLibrary|DoesDataTableRowExist "/Game/통합/Table/BP_DT_SelectTable.BP_DT_SelectTable" (Utilities|String|StringToName (Utilities|String|ToString(Integer) _array_element_2))))
    (if _returnvalue_2
      (bind _returnvalue_3 (Utilities|GetDataTableRow "/Game/통합/Table/BP_DT_SelectTable.BP_DT_SelectTable" (Utilities|String|StringToName (Utilities|String|ToString(Integer) _array_element_2)))
        (:then
          (Utilities|Array|Add (LocalVariables|GetList) (Utilities|Struct|MakeST_SelectData (.NextInteraction (Utilities|Struct|BreakTS_SelectTable _returnvalue_3)) (.ButtonText (Utilities|Struct|BreakTS_SelectTable _returnvalue_3)) self))))))
  (return (LocalVariables|GetList)))

(fn GenerateBubble
  (params (targetId :type Integer))
  (if (== (Variables|Default|GetScriptId) 0)
    (bind _output_get (Variables|Default|SetScriptId targetId))
    (elif (== (Variables|Default|GetScriptId) -1)
      (bind _returnvalue (Utilities|GetDataTableRow "/Game/통합/Table/BP_DT_NextInteraction.BP_DT_NextInteraction" (Utilities|String|StringToName (Utilities|String|ToString(Integer) (Variables|Default|GetScriptId))))
        (:then
          (Variables|Default|SetCurrentInteraction (Utilities|Struct|BreakTS_NextInteraction _returnvalue))
          (LocalVariables|SetReturnValue (Variables|Default|GetPreScriptId))
          (Variables|Default|SetPreScriptId 0)
          (Variables|Default|SetScriptId 0)
          (Variables|Default|SetIsScriptOver false)
          (return (LocalVariables|GetReturnValue))))
      (else
        _)))
  (bind _returnvalue_2 (Utilities|GetDataTableRow (Variables|Default|GetScriptTable) (Utilities|String|StringToName (Utilities|String|ToString(Integer) _output_get)))
    (:then
      (Default|StartAnimation (.AsBP%20UMG%20Bubble%20Widget (Utilities|Casting|CastToBP_UMG_BubbleWidget (UserInterface|GetWidget (Variables|Default|GetBubble)))) (.Name (Utilities|Struct|BreakTS_Script _returnvalue_2)) (.Script (Utilities|Struct|BreakTS_Script _returnvalue_2)))
      (if (== (.NextId (Utilities|Struct|BreakTS_Script _returnvalue_2)) 0)
        (bind _output_get_2 (Variables|Default|SetPreScriptId (Variables|Default|GetScriptId)))
        (Variables|Default|SetScriptId -1)
        (return _output_get_2)
        (else
          (bind _output_get_3 (Variables|Default|SetPreScriptId (Variables|Default|GetScriptId)))
          (bind _output_get_4 (Variables|Default|SetScriptId (.NextId (Utilities|Struct|BreakTS_Script _returnvalue_2))))
          (bind _returnvalue_3 (Utilities|GetDataTableRow "/Game/통합/Table/BP_DT_NextInteraction.BP_DT_NextInteraction" (Utilities|String|StringToName (Utilities|String|ToString(Integer) _output_get_4)))
            (:then
              (Variables|Default|SetCurrentInteraction (Utilities|Struct|BreakTS_NextInteraction _returnvalue_3))
              (return _output_get_3))))))))