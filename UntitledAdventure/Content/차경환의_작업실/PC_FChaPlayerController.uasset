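; Player controller for the FCha character, handling Enhanced Input movement, look, jump, sprint and interaction.
; Tick and movement input switch the pawn's CameraShakeSource between idle, walk and sprint shakes based on velocity.
; Sprint changes max walk speed, and Interact sends InteractionMessage to the first overlapping actor implementing the interaction interface unless IsSelecting is set.
; Setter events toggle the flags that gate movement, camera look and interaction.
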(event Input|EnhancedActionEvents|EnhancedInputActionIA_FChaForward
  (params (ActionValue :type Float%20%28double-precision%29) (ElapsedSeconds :type Float%20%28double-precision%29) (TriggeredSeconds :type Float%20%28double-precision%29) (InputAction :type Input%20Action%20Object%20Reference :default "/Game/차경환의_작업실/input/IA_FChaForward.IA_FChaForward"))
  (bind _returnvalue (Pawn|GetControlledPawn))
  (bind _returnvalue_2 (Actor|GetComponentbyClass _returnvalue "/Script/Engine.CameraShakeSourceComponent"))
  ;[1 1 1] 전진
  (:Triggered
    (if (Variables|Default|GetCharacterMovable)
      (Pawn|Input|AddMovementInput (Pawn|GetControlledPawn) (Math|Vector|GetForwardVector (Math|Rotator|MakeRotator 0.0 0.0 (.yaw (Pawn|GetControlRotation :!class /Script/Engine.Controller)))) ActionValue false)
      (if (> (Math|Vector|VectorLength (Variables|/Script/Engine.MovementComponent|GetVelocity (Actor|GetComponentbyClass (Pawn|GetControlledPawn) "/Script/Engine.CharacterMovementComponent"))) 3.1e+02)
        (Class|CameraShakeSourceComponent|StopAllCameraShakesOfType _returnvalue_2 "/Game/차경환의_작업실/BP_FchaCameraShake.BP_FchaCameraShake_C" false)
        (Class|CameraShakeSourceComponent|StopAllCameraShakesOfType _returnvalue_2 "/Game/차경환의_작업실/BP_FchaWalkCameraShake.BP_FchaWalkCameraShake_C" false)
        (CameraShakes|StartCameraShake _returnvalue_2 "/Game/차경환의_작업실/BP_FchaSprintCameraShake.BP_FchaSprintCameraShake_C" 1.0 "CameraLocal" "0, 0, 0")
        (else
          (Class|CameraShakeSourceComponent|StopAllCameraShakesOfType _returnvalue_2 "/Game/차경환의_작업실/BP_FchaCameraShake.BP_FchaCameraShake_C" false)
          (Class|CameraShakeSourceComponent|StopAllCameraShakesOfType _returnvalue_2 "/Game/차경환의_작업실/BP_FchaSprintCameraShake.BP_FchaSprintCameraShake_C" false)
          (CameraShakes|StartCameraShake _returnvalue_2 "/Game/차경환의_작업실/BP_FchaWalkCameraShake.BP_FchaWalkCameraShake_C" 1.0 "CameraLocal" "0, 0, 0"))))))

(event Input|EnhancedActionEvents|EnhancedInputActionIA_FChaRight
  (params (ActionValue :type Float%20%28double-precision%29) (ElapsedSeconds :type Float%20%28double-precision%29) (TriggeredSeconds :type Float%20%28double-precision%29) (InputAction :type Input%20Action%20Object%20Reference :default "/Game/차경환의_작업실/input/IA_FChaRight.IA_FChaRight"))
  (bind _returnvalue (Pawn|GetControlledPawn))
  (bind _returnvalue_2 (Pawn|GetControlRotation :!class /Script/Engine.Controller))
  (bind _returnvalue_3 (Actor|GetComponentbyClass _returnvalue "/Script/Engine.CameraShakeSourceComponent"))
  ;[1 1 1] 좌우 이동
  (:Triggered
    (if (Variables|Default|GetCharacterMovable)
      (Pawn|Input|AddMovementInput (Pawn|GetControlledPawn) (Math|Vector|GetRightVector (Math|Rotator|MakeRotator (.roll _returnvalue_2) 0.0 (.yaw _returnvalue_2))) ActionValue false)
      (if (> (Math|Vector|VectorLength (Variables|/Script/Engine.MovementComponent|GetVelocity (Actor|GetComponentbyClass (Pawn|GetControlledPawn) "/Script/Engine.CharacterMovementComponent"))) 3.1e+02)
        (Class|CameraShakeSourceComponent|StopAllCameraShakesOfType _returnvalue_3 "/Game/차경환의_작업실/BP_FchaCameraShake.BP_FchaCameraShake_C" false)
        (Class|CameraShakeSourceComponent|StopAllCameraShakesOfType _returnvalue_3 "/Game/차경환의_작업실/BP_FchaWalkCameraShake.BP_FchaWalkCameraShake_C" false)
        (CameraShakes|StartCameraShake _returnvalue_3 "/Game/차경환의_작업실/BP_FchaSprintCameraShake.BP_FchaSprintCameraShake_C" 1.0 "CameraLocal" "0, 0, 0")
        (else
          (Class|CameraShakeSourceComponent|StopAllCameraShakesOfType _returnvalue_3 "/Game/차경환의_작업실/BP_FchaCameraShake.BP_FchaCameraShake_C" false)
          (Class|CameraShakeSourceComponent|StopAllCameraShakesOfType _returnvalue_3 "/Game/차경환의_작업실/BP_FchaSprintCameraShake.BP_FchaSprintCameraShake_C" false)
          (CameraShakes|StartCameraShake _returnvalue_3 "/Game/차경환의_작업실/BP_FchaWalkCameraShake.BP_FchaWalkCameraShake_C" 1.0 "CameraLocal" "0, 0, 0"))))))

(event Input|EnhancedActionEvents|EnhancedInputActionIA_FChaLookup
  (params (ActionValue :type Float%20%28double-precision%29) (ElapsedSeconds :type Float%20%28double-precision%29) (TriggeredSeconds :type Float%20%28double-precision%29) (InputAction :type Input%20Action%20Object%20Reference :default "/Game/차경환의_작업실/input/IA_FChaLookup.IA_FChaLookup"))
  ;[1 1 1] 카메라 회전
  (:Triggered
    (if (Variables|Default|GetCameraMovable)
      (Class|PlayerController|AddPitchInput ActionValue))))

(event Input|EnhancedActionEvents|EnhancedInputActionIA_FChaLookRight
  (params (ActionValue :type Float%20%28double-precision%29) (ElapsedSeconds :type Float%20%28double-precision%29) (TriggeredSeconds :type Float%20%28double-precision%29) (InputAction :type Input%20Action%20Object%20Reference :default "/Game/차경환의_작업실/input/IA_FChaLookRight.IA_FChaLookRight"))
  ;[1 1 1] 카메라 회전
  (:Triggered
    (if (Variables|Default|GetCameraMovable)
      (Class|PlayerController|AddYawInput ActionValue))))

(event Input|EnhancedActionEvents|EnhancedInputActionIA_FChaJump
  (params (ActionValue :type Boolean) (ElapsedSeconds :type Float%20%28double-precision%29) (TriggeredSeconds :type Float%20%28double-precision%29) (InputAction :type Input%20Action%20Object%20Reference :default "/Game/차경환의_작업실/input/IA_FChaJump.IA_FChaJump"))
  (bind _returnvalue (Pawn|GetControlledPawn))
  (bind _asbp_fcha_base_character (Utilities|Casting|CastToBP_FChaBaseCharacter _returnvalue))
  ;[1 1 1] 점프
  (:Started
    (Character|Jump _asbp_fcha_base_character))
  (:Completed
    (Character|StopJumping _asbp_fcha_base_character)))

(event Input|EnhancedActionEvents|EnhancedInputActionIA_FChaSprint
  (params (ActionValue :type Boolean) (ElapsedSeconds :type Float%20%28double-precision%29) (TriggeredSeconds :type Float%20%28double-precision%29) (InputAction :type Input%20Action%20Object%20Reference :default "/Game/차경환의_작업실/input/IA_FChaSprint.IA_FChaSprint"))
  (bind _returnvalue (Pawn|GetControlledPawn))
  (bind _returnvalue_2 (Actor|GetComponentbyClass _returnvalue "/Script/Engine.CharacterMovementComponent"))
  ;[1 1 1] 달리기
  (:Started
    (Variables|/Script/Engine.CharacterMovementComponent|SetMaxWalkSpeed _returnvalue_2 6e+02))
  (:Completed
    (Variables|/Script/Engine.CharacterMovementComponent|SetMaxWalkSpeed _returnvalue_2 3e+02)))

(event Input|EnhancedActionEvents|EnhancedInputActionIA_FChaInteract
  (params (ActionValue :type Boolean) (ElapsedSeconds :type Float%20%28double-precision%29) (TriggeredSeconds :type Float%20%28double-precision%29) (InputAction :type Input%20Action%20Object%20Reference :default "/Game/차경환의_작업실/input/IA_FChaInteract.IA_FChaInteract"))
  (:Started
    (if (not (Variables|Default|GetIs%20Selecting))
      (bind _array_element (Utilities|Array|ForEachLoopwithBreak (Collision|GetOverlappingActors (Pawn|GetControlledPawn self) "/Script/Engine.Actor" :!class /Script/Engine.Actor) :!label _label)
        (:LoopBody
          (if (Utilities|DoesObjectImplementInterface _array_element "/Game/통합/Interface/BP_ATI_InteractionWithActor.BP_ATI_InteractionWithActor_C")
            (Class|BPATIInteractionwithActor|Interaction(Message) _array_element)
            (goto _label Break)))))))

(event EventBeginPlay
  (bind _self self)
  (bind _returnvalue (PlayerController|LocalPlayerSubsystems|GetEnhancedInputLocalPlayerSubsystem _self))
  (Utilities|IsValid _returnvalue
    (:Is%20Valid
      (Input|AddMappingContext _returnvalue "/Game/차경환의_작업실/input/IMC_FChaIMC.IMC_FChaIMC" 0 "(bIgnoreAllPressedKeysUntilRelease=True,bForceImmediately=False)"))))

(event EventTick
  (params (DeltaSeconds :type Float%20%28single-precision%29))
  (bind _returnvalue (Pawn|GetControlledPawn))
  (bind _returnvalue_2 (Actor|GetComponentbyClass _returnvalue "/Script/Engine.CameraShakeSourceComponent"))
  ;[1 1 1] 카메라 쉐이크 조정
  (if (== 0.0 (Math|Vector|VectorLength (Variables|/Script/Engine.MovementComponent|GetVelocity (Actor|GetComponentbyClass (Pawn|GetControlledPawn) "/Script/Engine.CharacterMovementComponent"))))
    (Class|CameraShakeSourceComponent|StopAllCameraShakesOfType _returnvalue_2 "/Game/차경환의_작업실/BP_FchaWalkCameraShake.BP_FchaWalkCameraShake_C" false)
    (Class|CameraShakeSourceComponent|StopAllCameraShakesOfType _returnvalue_2 "/Game/차경환의_작업실/BP_FchaSprintCameraShake.BP_FchaSprintCameraShake_C" false)
    (CameraShakes|StartCameraShake _returnvalue_2 "/Game/차경환의_작업실/BP_FchaCameraShake.BP_FchaCameraShake_C" 1.0 "CameraLocal" "0, 0, 0")))

(event EventIsSelecting
  (params (IsSelecting :type Boolean))
  (Variables|Default|SetIs%20Selecting IsSelecting))

(event EventControllerHoldSet
  (params (Set :type Boolean))
  (Variables|Default|SetCharacterMovable Set))

(event EventCameraHoldSet
  (params (Set :type Boolean))
  (Variables|Default|SetCameraMovable Set))

(fn ConstructionScript)