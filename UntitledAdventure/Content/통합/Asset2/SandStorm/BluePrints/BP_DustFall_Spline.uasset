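; Placeable spline-based dust fall effect that drives a Niagara system along an editable spline.
; The construction script passes the spline and exposed actor variables into the SplineDustFall component as user parameters.
; A smoke type selector swaps the first layer's material, while four smoke layers get spawn rate, colors, lifetime, size, emissive and contrast, plus velocity, noise and normal settings.
; There is no runtime logic, as the event graph is empty.
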(event EventBeginPlay)

(event Collision|EventActorBeginOverlap
  (params (OtherActor :type Actor%20Object%20Reference)))

(event EventTick
  (params (DeltaSeconds :type Float%20%28single-precision%29)))

(fn ConstructionScript
  (bind _splinedustfall (Variables|Default|GetSplineDustFall))
  (bind _splinedustfall_2 (Variables|Default|GetSplineDustFall))
  (bind _splinedustfall_3 (Variables|Default|GetSplineDustFall))
  (bind _splinedustfall_4 (Variables|Default|GetSplineDustFall))
  (bind _splinedustfall_5 (Variables|Default|GetSplineDustFall))
  ;[0.9468 0 1 1 100] Set Niagara Parameters
  (Class|NiagaraComponent|SetVariableObject (Variables|Default|GetSplineDustFall) "Spline" (Variables|Default|GetSpline))
  (switch Utilities|FlowControl|Switch|SwitchonSmokeType (Variables|Smoke_A|GetSmokeType1)
    (:NewEnumerator0
      (Class|NiagaraComponent|SetVariableMaterial _splinedustfall_5 "mat1" "/Game/통합/Asset2/SandStorm/Materials/MI_MV_Smoke_Inst4.MI_MV_Smoke_Inst4"))
    (:NewEnumerator1
      (Class|NiagaraComponent|SetVariableMaterial _splinedustfall_5 "mat1" "/Game/통합/Asset2/SandStorm/Materials/MI_MV_Smoke_Inst6.MI_MV_Smoke_Inst6"))
    (:NewEnumerator2
      (Class|NiagaraComponent|SetVariableMaterial _splinedustfall_5 "mat1" "/Game/통합/Asset2/SandStorm/Materials/MI_MV_Smoke_Inst7.MI_MV_Smoke_Inst7")))
  (Niagara|SetNiagaraVariable(Float) _splinedustfall "SpawnRate1" (Variables|Smoke_A|GetSpawnRate1))
  (Niagara|SetNiagaraVariable(LinearColor) _splinedustfall "Color_SmokeA" (Variables|Smoke_A|GetColor_A1))
  (Niagara|SetNiagaraVariable(LinearColor) _splinedustfall "Color_SmokeB" (Variables|Smoke_A|GetColor_B1))
  (Niagara|SetNiagaraVariable(Float) _splinedustfall "LifetimeA" (Variables|Smoke_A|GetLifetime1))
  (Niagara|SetNiagaraVariable(Float) _splinedustfall "Scale_SizeA" (Variables|Smoke_A|GetScale_Size1))
  (Niagara|SetNiagaraVariable(Float) _splinedustfall "EmessiveA" (Variables|Smoke_A|GetEmessive1))
  (Niagara|SetNiagaraVariable(Float) _splinedustfall "Contrast_A" (Variables|Smoke_A|GetContrast1))
  (Niagara|SetNiagaraVariable(Float) _splinedustfall_4 "SpawnRate2" (Variables|Smoke_B|GetSpawnRate2))
  (Niagara|SetNiagaraVariable(LinearColor) _splinedustfall_4 "Color_SmokeA2" (Variables|Smoke_B|GetColor_A2))
  (Niagara|SetNiagaraVariable(LinearColor) _splinedustfall_4 "Color_SmokeB2" (Variables|Smoke_B|GetColor_B2))
  (Niagara|SetNiagaraVariable(Float) _splinedustfall_4 "LifetimeB" (Variables|Smoke_B|GetLifetime2))
  (Niagara|SetNiagaraVariable(Float) _splinedustfall_4 "ScaleSize_B" (Variables|Smoke_B|GetScale_Size2))
  (Niagara|SetNiagaraVariable(Float) _splinedustfall_4 "EmessiveB" (Variables|Smoke_B|GetEmessive2))
  (Niagara|SetNiagaraVariable(Float) _splinedustfall_4 "Contrast_B" (Variables|Smoke_B|GetContrast2))
  (Niagara|SetNiagaraVariable(Float) _splinedustfall_4 "Velocity2" (Variables|Smoke_B|GetVelocity2))
  (Niagara|SetNiagaraVariable(Float) _splinedustfall_3 "SpawnRate3" (Variables|Particles|GetSpawnRate3))
  (Niagara|SetNiagaraVariable(LinearColor) _splinedustfall_3 "Color_SmokeA3" (Variables|Particles|GetColor_A3))
  (Niagara|SetNiagaraVariable(LinearColor) _splinedustfall_3 "Color_SmokeB3" (Variables|Particles|GetColor_B3))
  (Niagara|SetNiagaraVariable(Float) _splinedustfall_3 "LifetimeC" (Variables|Particles|GetLifetime3))
  (Niagara|SetNiagaraVariable(Float) _splinedustfall_3 "ScaleSize_C" (Variables|Particles|GetScale_Size3))
  (Niagara|SetNiagaraVariable(Float) _splinedustfall_3 "EmessiveC" (Variables|Particles|GetEmessive3))
  (Niagara|SetNiagaraVariable(Float) _splinedustfall_3 "Contrast_C" (Variables|Particles|GetContrast3))
  (Niagara|SetNiagaraVariable(Float) _splinedustfall_3 "Velocity3" (Variables|Particles|GetVelocity3))
  (Niagara|SetNiagaraVariable(Float) _splinedustfall_3 "Noise Strength" (Variables|Particles|GetNoise%20Strength))
  (Niagara|SetNiagaraVariable(Float) _splinedustfall_3 "Noise Frequency" (Variables|Particles|GetNoise%20Frequency))
  (Niagara|SetNiagaraVariable(Float) _splinedustfall_2 "SpawnRate4" (Variables|Smoke_C|GetSpawnRate4))
  (Niagara|SetNiagaraVariable(LinearColor) _splinedustfall_2 "Color_SmokeA4" (Variables|Smoke_C|GetColor_A4))
  (Niagara|SetNiagaraVariable(LinearColor) _splinedustfall_2 "Color_SmokeB4" (Variables|Smoke_C|GetColor_B4))
  (Niagara|SetNiagaraVariable(Float) _splinedustfall_2 "LifetimeD" (Variables|Smoke_C|GetLifetime4))
  (Niagara|SetNiagaraVariable(Float) _splinedustfall_2 "ScaleSize_D" (Variables|Smoke_C|GetScale_Size4))
  (Niagara|SetNiagaraVariable(Float) _splinedustfall_2 "EmessiveD" (Variables|Smoke_C|GetEmessive4))
  (Niagara|SetNiagaraVariable(Float) _splinedustfall_2 "Contrast_D" (Variables|Smoke_C|GetContrast4))
  (Niagara|SetNiagaraVariable(Float) _splinedustfall_2 "Velocity4" (Variables|Smoke_C|GetVelocity4))
  (Niagara|SetNiagaraVariable(Float) (Variables|Default|GetSplineDustFall) "NormalIntensity" (Variables|ToAll|GetNormalIntensity)))