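; Placeable sandstorm actor that lays a surface layer of animated dust over the ground, built entirely in the Construction Script.
; It spawns a centered, non-colliding grid of the chosen mesh sized by AreaResolution and Scale, then sphere-traces each tile down to snap and align it to the surface below.
; Each tile gets a dynamic material with the selected dust textures and exposed look parameters.
; Alpha, height offset and contrast are adjusted toward the box edges to fade the borders.
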(event EventBeginPlay)

(event Collision|EventActorBeginOverlap
  (params (OtherActor :type Actor%20Object%20Reference)))

(event EventTick
  (params (DeltaSeconds :type Float%20%28single-precision%29)))

(fn ConstructionScript
  (bind _arrow (Variables|Default|GetArrow))
  (bind _box (Variables|Default|GetBox))
  (bind _arearesolution (Variables|Basic|GetAreaResolution))
  (bind _arearesolution_2 (Variables|Basic|GetAreaResolution))
  (bind _arearesolution_3 (Variables|Basic|GetAreaResolution))
  (bind (_x _y) (Math|Vector2D|BreakVector2D _arearesolution_3))
  (bind (_x_2 _y_2) (Math|Vector2D|BreakVector2D _arearesolution))
  (bind (_x_3 _y_3) (Math|Vector2D|BreakVector2D _arearesolution_2))
  ;[0.3026 0 1 1 100] Set Scale
  (Transformation|SetWorldScale3D (Variables|Default|GetDefaultSceneRoot) (Math|Conversions|ToVector(Float) (Variables|Basic|GetScale)))
  (Variables|Default|SetArea (* (.X (Math|Vector|BreakVector (.BoxExtent (Math|BoxSphereBounds|BreakBoxSphereBounds (StaticMesh|GetBounds (Variables|Default|GetStaticmesh)))))) 2.0 (Variables|Basic|GetScale)))
  (Transformation|SetAbsolute (Variables|Default|GetBox) false true false)
  ;[1 0 0.7085 1 100] Set Box Collision Location
  (Variables|Default|SetBoxExtent (Math|Vector|MakeVector (* _x (* (Variables|Default|GetArea) 0.5 (/ 1.0 (Variables|Basic|GetScale)))) (* _y (* (Variables|Default|GetArea) 0.5 (/ 1.0 (Variables|Basic|GetScale)))) (* 5.0 (* (Variables|Default|GetArea) 0.5 (/ 1.0 (Variables|Basic|GetScale))))))
  (Components|Box|SetBoxExtent _box (Variables|Default|GetBoxExtent) true)
  (Transformation|SetRelativeLocation _box (Math|Vector|MakeVector 0.0 0.0 (* (* 5.0 (* (Variables|Default|GetArea) 0.5 (/ 1.0 (Variables|Basic|GetScale)))) -1.0)) false false)
  (switch Utilities|FlowControl|Switch|SwitchonDustSurface_Mesh_Type (Variables|Basic|GetMeshType)
    (:NewEnumerator0
      (Variables|Default|SetStaticmesh "/Game/통합/Asset2/SandStorm/Meshes/SM_Grid_00.SM_Grid_00"))
    (:NewEnumerator1
      (Variables|Default|SetStaticmesh "/Game/통합/Asset2/SandStorm/Meshes/SM_Grid_01.SM_Grid_01"))
    (:NewEnumerator2
      (Variables|Default|SetStaticmesh "/Game/통합/Asset2/SandStorm/Meshes/SM_Grid_02.SM_Grid_02"))
    (:NewEnumerator3
      (Variables|Default|SetStaticmesh "/Game/통합/Asset2/SandStorm/Meshes/SM_Grid_03.SM_Grid_03")))
  ;[1 0.077 0 1 100] Add Static mesh Component
  (for _index (range 1 (Math|Float|Truncate (* (Math|Float|Absolute(Float) _x_2) (Math|Float|Absolute(Float) _y_2))))
    (bind _returnvalue (AddComponent|AddStaticMeshComponent false (Math|Transform|MakeTransform "0, 0, 0")))
    (Components|StaticMesh|SetStaticMesh _returnvalue (Variables|Default|GetStaticmesh))
    (Transformation|SetRelativeScale3D _returnvalue (Math|Conversions|ToVector(Float) (Variables|Basic|GetOverlap)))
    (Utilities|Array|SetArrayElem (Variables|Default|GetGrid) _index _returnvalue true))
  ;[1 0.374 0 1 100] Set Static Mesh Location
  (for (_array_element _array_index) (Variables|Default|GetGrid)
    (Utilities|IsValid _array_element
      (:Is%20Valid
        (Transformation|AddRelativeLocation _array_element (Math|Vector|MakeVector (* (Math|Integer|%(Integer) _array_index (Math|Float|Truncate (Math|Float|Absolute(Float) (.X (Math|Vector2D|BreakVector2D (Variables|Basic|GetAreaResolution)))))) (Variables|Default|GetArea)) (* (Variables|Default|Getplus) (Variables|Default|GetArea)) 0.0) false false)
        (if (and (> _array_index 0) (== (Math|Integer|%(Integer) _array_index (Math|Float|Truncate (Math|Float|Absolute(Float) (.X (Math|Vector2D|BreakVector2D (Variables|Basic|GetAreaResolution)))))) 0))
          (bind _result (Math|Integer|IncrementInt (Variables|Default|Getplus))
            (:%20%20
              (Variables|Default|Setplus _result)))))))
  ;[1 0.8092 0 1 100] offset Static Mesh Location
  (for _array_element_2 (Variables|Default|GetGrid)
    (Utilities|IsValid _array_element_2
      (:Is%20Valid
        (Transformation|AddRelativeLocation _array_element_2 (Math|Vector|MakeVector (* (* (- (Math|Float|Truncate (Math|Float|Absolute(Float) _x_3)) 1) (Variables|Default|GetArea)) -0.5) (* (* (- (Math|Float|Truncate (Math|Float|Absolute(Float) _y_3)) 1) (Variables|Default|GetArea)) -0.5) 0.0) false false))))
  ;[0.4606 1 0 1 100] Set up Sphere Trace Channel
  (for _array_element_3 (Variables|Default|GetGrid)
    (Utilities|IsValid _array_element_3
      (:Is%20Valid
        (bind (_outhit _returnvalue_2) (Collision|SphereTraceByChannel (+ (Variables|/Script/Engine.SceneComponent|GetRelativeLocation _array_element_3) (Transformation|GetWorldLocation _arrow)) (+ (+ (Variables|/Script/Engine.SceneComponent|GetRelativeLocation _array_element_3) (Transformation|GetWorldLocation _arrow)) (* (Math|Vector|GetUpVector _arrow) (Math|Conversions|ToVector(Float) -1e+03))) 2e+01 "TraceTypeQuery1" true 0 "None"))
        (if _returnvalue_2
          (Transformation|SetWorldLocation _array_element_3 (.Location (Collision|BreakHitResult _outhit)) false false)
          (Transformation|SetWorldRotation _array_element_3 (Math|Rotator|MakeRotfromZX (Math|Vector|Normalize (.ImpactNormal (Collision|BreakHitResult _outhit))) (Math|Vector|GetForwardVector _array_element_3)) false false)))))
  ;[0 1 0.4337 1 100] Set Material
  (for _array_element_4 (Variables|Default|GetGrid)
    (Utilities|IsValid _array_element_4
      (:Is%20Valid
        (bind _returnvalue_3 (Rendering|Material|CreateDynamicMaterialInstance _array_element_4 0 "/Game/통합/Asset2/SandStorm/Materials/MI_OnSurface_Inst.MI_OnSurface_Inst" "None" :!class /Script/Engine.PrimitiveComponent))
        (Collision|SetCollisionEnabled _array_element_4 "NoCollision")
        (switch Utilities|FlowControl|Switch|SwitchonDustSurface_Smoke_Type (Variables|Basic|GetDustType)
          (:NewEnumerator0
            (Rendering|Material|SetTextureParameterValue _returnvalue_3 "CM" "/Game/통합/Asset2/SandStorm/Textures/T_C_Cam11.T_C_Cam11")
            (Rendering|Material|SetTextureParameterValue _returnvalue_3 "MVC" "/Game/통합/Asset2/SandStorm/Textures/T_MV_Cam11.T_MV_Cam11")
            (Rendering|Material|SetTextureParameterValue _returnvalue_3 "NM" "/Game/통합/Asset2/SandStorm/Textures/T_N_Cam11.T_N_Cam11"))
          (:NewEnumerator1
            (Rendering|Material|SetTextureParameterValue _returnvalue_3 "CM" "/Game/통합/Asset2/SandStorm/Textures/T_C_Cam111.T_C_Cam111")
            (Rendering|Material|SetTextureParameterValue _returnvalue_3 "MVC" "/Game/통합/Asset2/SandStorm/Textures/T_MV_Cam111.T_MV_Cam111")
            (Rendering|Material|SetTextureParameterValue _returnvalue_3 "NM" "/Game/통합/Asset2/SandStorm/Textures/T_N_Cam111.T_N_Cam111"))
          (:NewEnumerator2
            (Rendering|Material|SetTextureParameterValue _returnvalue_3 "CM" "/Game/통합/Asset2/SandStorm/Textures/T_C_Cam1111.T_C_Cam1111")
            (Rendering|Material|SetTextureParameterValue _returnvalue_3 "MVC" "/Game/통합/Asset2/SandStorm/Textures/T_MV_Cam1111.T_MV_Cam1111")
            (Rendering|Material|SetTextureParameterValue _returnvalue_3 "NM" "/Game/통합/Asset2/SandStorm/Textures/T_N_Cam1111.T_N_Cam1111"))
          (:NewEnumerator3
            (Rendering|Material|SetTextureParameterValue _returnvalue_3 "CM" "/Game/통합/Asset2/SandStorm/Textures/T_C_Cam11111.T_C_Cam11111")
            (Rendering|Material|SetTextureParameterValue _returnvalue_3 "MVC" "/Game/통합/Asset2/SandStorm/Textures/T_MV_Cam11111.T_MV_Cam11111")
            (Rendering|Material|SetTextureParameterValue _returnvalue_3 "NM" "/Game/통합/Asset2/SandStorm/Textures/T_N_Cam11111.T_N_Cam11111"))
          (:NewEnumerator4
            (Rendering|Material|SetTextureParameterValue _returnvalue_3 "CM" "/Game/통합/Asset2/SandStorm/Textures/T_C_Cam111111.T_C_Cam111111")
            (Rendering|Material|SetTextureParameterValue _returnvalue_3 "MVC" "/Game/통합/Asset2/SandStorm/Textures/T_MV_Cam111111.T_MV_Cam111111")
            (Rendering|Material|SetTextureParameterValue _returnvalue_3 "NM" "/Game/통합/Asset2/SandStorm/Textures/T_N_Cam111111.T_N_Cam111111"))))))
  ;[0 0.9048 1 1 100] Set Material Parameters
  (for _array_element_5 (Variables|Default|GetGrid)
    (Utilities|IsValid _array_element_5
      (:Is%20Valid
        (Rendering|Material|SetScalarParameterValueonMaterials _array_element_5 "Rotate" (+ (Math|Float|MapRangeClamped (.Yaw (Math|Rotator|BreakRotator (Transformation|GetWorldRotation (Variables|Default|GetDefaultSceneRoot)))) -3.6e+02 3.6e+02 1.0 -1.0) -0.25))
        (Rendering|Material|SetScalarParameterValueonMaterials _array_element_5 "DotPower" (Variables|Basic|GetDepth))
        (Rendering|Material|SetVectorParameterValueonMaterials _array_element_5 "BC" (Math|Conversions|ToVector(LinearColor) (Variables|Basic|GetBaseColor)))
        (Rendering|Material|SetScalarParameterValueonMaterials _array_element_5 "Power" (Variables|Dust|GetContrast))
        (Rendering|Material|SetVectorParameterValueonMaterials _array_element_5 "Color" (Math|Conversions|ToVector(LinearColor) (Variables|Dust|GetColor)))
        (Rendering|Material|SetScalarParameterValueonMaterials _array_element_5 "Alpha" (Variables|Dust|GetAlpha))
        (Rendering|Material|SetScalarParameterValueonMaterials _array_element_5 "TileDivide" (* (Variables|Dust|GetTileScale) 1e+04 (Variables|Basic|GetScale)))
        (Rendering|Material|SetScalarParameterValueonMaterials _array_element_5 "PannerSpeed" (Variables|Dust|GetMoveSpeed))
        (Rendering|Material|SetScalarParameterValueonMaterials _array_element_5 "Speed" (Variables|Dust|GetDustSpeed))
        (Rendering|Material|SetScalarParameterValueonMaterials _array_element_5 "Normal" (Variables|Dust|GetNormalMapIntensity))
        (Rendering|Material|SetScalarParameterValueonMaterials _array_element_5 "Depthfade" (Variables|Dust|GetDepthFade))
        (Rendering|Material|SetScalarParameterValueonMaterials _array_element_5 "Emessive" (Variables|Dust|GetEmessive))
        (Rendering|Material|SetScalarParameterValueonMaterials _array_element_5 "SandNoiseScale" (Variables|Dust|GetSandNoiseScale))
        (Rendering|Material|SetScalarParameterValueonMaterials _array_element_5 "SandNoise" (Variables|Dust|GetSandLerp))
        (Rendering|Material|SetScalarParameterValueonMaterials _array_element_5 "OffsetHeight" (Variables|Basic|GetHeightOffset)))))
  ;[0.1009 1 0.2975 1 100] Fade Setup
  (for _array_element_6 (Variables|Default|GetGrid)
    (Utilities|IsValid _array_element_6
      (:Is%20Valid
        (Rendering|Material|SetScalarParameterValueonMaterials _array_element_6 "Alpha" (* (Math|Float|MapRangeClamped (Math|Float|Absolute(Float) (.X (Math|Vector|BreakVector (Variables|/Script/Engine.SceneComponent|GetRelativeLocation _array_element_6)))) (- (.X (Math|Vector|BreakVector (Variables|Default|GetBoxExtent))) (Math|Float|Lerp 0.0 (.X (Math|Vector|BreakVector (Variables|Default|GetBoxExtent))) (Variables|Dust|GetXDirection_Fade))) (.X (Math|Vector|BreakVector (Variables|Default|GetBoxExtent))) 1.0 0.0) (Variables|Dust|GetAlpha) (Math|Float|MapRangeClamped (Math|Float|Absolute(Float) (.Y (Math|Vector|BreakVector (Variables|/Script/Engine.SceneComponent|GetRelativeLocation _array_element_6)))) (- (.Y (Math|Vector|BreakVector (Variables|Default|GetBoxExtent))) (Math|Float|Lerp 0.0 (.Y (Math|Vector|BreakVector (Variables|Default|GetBoxExtent))) (Variables|Dust|GetYDirection_Fade))) (.Y (Math|Vector|BreakVector (Variables|Default|GetBoxExtent))) 1.0 0.0)))
        (Rendering|Material|SetScalarParameterValueonMaterials _array_element_6 "OffsetHeight" (* (Math|Float|MapRangeClamped (Math|Float|Absolute(Float) (.X (Math|Vector|BreakVector (Variables|/Script/Engine.SceneComponent|GetRelativeLocation _array_element_6)))) (- (.X (Math|Vector|BreakVector (Variables|Default|GetBoxExtent))) (Math|Float|Lerp 0.0 (.X (Math|Vector|BreakVector (Variables|Default|GetBoxExtent))) (Variables|Dust|GetXDirection_Fade))) (.X (Math|Vector|BreakVector (Variables|Default|GetBoxExtent))) 1.0 0.0) (Math|Float|MapRangeClamped (Math|Float|Absolute(Float) (.Y (Math|Vector|BreakVector (Variables|/Script/Engine.SceneComponent|GetRelativeLocation _array_element_6)))) (- (.Y (Math|Vector|BreakVector (Variables|Default|GetBoxExtent))) (Math|Float|Lerp 0.0 (.Y (Math|Vector|BreakVector (Variables|Default|GetBoxExtent))) (Variables|Dust|GetYDirection_Fade))) (.Y (Math|Vector|BreakVector (Variables|Default|GetBoxExtent))) 1.0 0.0) (Variables|Basic|GetHeightOffset)))
        (Rendering|Material|SetScalarParameterValueonMaterials _array_element_6 "Power" (* (Math|Float|MapRangeClamped (* (Math|Float|MapRangeClamped (Math|Float|Absolute(Float) (.X (Math|Vector|BreakVector (Variables|/Script/Engine.SceneComponent|GetRelativeLocation _array_element_6)))) (- (.X (Math|Vector|BreakVector (Variables|Default|GetBoxExtent))) (Math|Float|Lerp 0.0 (.X (Math|Vector|BreakVector (Variables|Default|GetBoxExtent))) (Variables|Dust|GetXDirection_Fade))) (.X (Math|Vector|BreakVector (Variables|Default|GetBoxExtent))) 1.0 0.0) (Math|Float|MapRangeClamped (Math|Float|Absolute(Float) (.Y (Math|Vector|BreakVector (Variables|/Script/Engine.SceneComponent|GetRelativeLocation _array_element_6)))) (- (.Y (Math|Vector|BreakVector (Variables|Default|GetBoxExtent))) (Math|Float|Lerp 0.0 (.Y (Math|Vector|BreakVector (Variables|Default|GetBoxExtent))) (Variables|Dust|GetYDirection_Fade))) (.Y (Math|Vector|BreakVector (Variables|Default|GetBoxExtent))) 1.0 0.0)) 1.0 0.0 1.0 2.0) (Variables|Dust|GetContrast)))))))