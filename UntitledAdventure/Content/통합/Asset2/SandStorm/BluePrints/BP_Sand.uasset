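; BP_Sand is a placeable sand effect actor from the SandStorm asset, wrapping a Sand Niagara component with tunable settings.
; Its construction script pushes the Blueprint variables into the Niagara user parameters, covering spawn rates for smoke, sand and particles, plus scale, lifetime, length, color range, emissive, contrast and distance fade.
; The event graph holds only disabled stubs, so the Blueprint adds no runtime logic.
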(event EventBeginPlay)

(event Collision|EventActorBeginOverlap
  (params (OtherActor :type Actor%20Object%20Reference)))

(event EventTick
  (params (DeltaSeconds :type Float%20%28single-precision%29)))

(fn ConstructionScript
  (bind _sand (Variables|Default|GetSand))
  ;[0 1 0.4314 1 100] Set Niagara Parameters
  (Niagara|SetNiagaraVariable(Float) _sand "SmokeSpawnRate" (Variables|Smoke|GetSmokeSpawnRate))
  (Niagara|SetNiagaraVariable(Float) _sand "SandSmokeSpawnRate" (Variables|SandSmoke|GetSandSmokeSpawnRate))
  (Niagara|SetNiagaraVariable(Float) _sand "SandScale" (Variables|Sand|GetSandScale))
  (Niagara|SetNiagaraVariable(Float) _sand "Sand_SpawnRate" (Variables|Sand|GetSand_SpawnRate))
  (Niagara|SetNiagaraVariable(Float) _sand "ParticleSpawnRate" (Variables|particles|GetParticleSpawnRate))
  (Niagara|SetNiagaraVariable(Float) _sand "ParticleSmokeSizeScale" (Variables|Basic|GetParticleSmokeSizeScale))
  (Niagara|SetNiagaraVariable(Float) _sand "Lifetime_Scale" (Variables|Basic|GetLifetime_Scale))
  (Niagara|SetNiagaraVariable(Float) _sand "Length" (Variables|Basic|GetLength))
  (Niagara|SetNiagaraVariable(Float) _sand "Emessive" (Variables|Basic|GetEmessive))
  (Niagara|SetNiagaraVariable(Float) _sand "Contrast" (Variables|Basic|GetContrast))
  (Niagara|SetNiagaraVariable(Float) _sand "AddWhiteColor" (Variables|Basic|GetAddWhiteColor))
  (Niagara|SetNiagaraVariable(Float) _sand "FadeDistance" (Variables|Basic|GetFadeDistance))
  (Niagara|SetNiagaraVariable(LinearColor) _sand "Color Minimum" (Variables|Basic|GetColor%20Minimum))
  (Niagara|SetNiagaraVariable(LinearColor) _sand "Color Maximum" (Variables|Basic|GetColor%20Maximum)))