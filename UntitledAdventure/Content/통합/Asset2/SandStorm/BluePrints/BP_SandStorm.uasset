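; Configurable sandstorm effect actor that wraps a Niagara system with a guide-driven Control Rig.
; The construction script pushes scale, smoke texture sets for start, middle and end stages, and look and motion parameters into Niagara, plus preview toggles.
; Five guide components map to Control Rig controls that drive the skeletal mesh.
; BeginPlay restarts the effect and, with FastSimulation on, uses a timeline to advance the simulation.
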(event EventBeginPlay
  ;[1 0.6127 0 1 100] Fast Simulation Set Up
  (Components|Activation|SetActive (Variables|Default|GetSandStorm) true true)
  (if (Variables|Basic|GetFastSimulation)
    (bind _newtrack_0 (Timeline|Timeline_1 Play)
      (:Update
        (Class|NiagaraComponent|AdvanceSimulationbyTime (Variables|Default|GetSandStorm) _newtrack_0 (Utilities|Time|GetWorldDeltaSeconds))))))

(event Collision|EventActorBeginOverlap
  (params (OtherActor :type Actor%20Object%20Reference)))

(event EventTick
  (params (DeltaSeconds :type Float%20%28single-precision%29)))

(fn ConstructionScript
  (bind _sandstorm (Variables|Default|GetSandStorm))
  (bind _sandstorm_2 (Variables|Default|GetSandStorm))
  (bind _sandstorm_3 (Variables|Default|GetSandStorm))
  (bind _sandstorm_4 (Variables|Default|GetSandStorm))
  (bind _sandstorm_5 (Variables|Default|GetSandStorm))
  (bind _scale (Variables|Basic|GetScale))
  (bind _sandstorm_6 (Variables|Default|GetSandStorm))
  (bind _sandstorm_7 (Variables|Default|GetSandStorm))
  (bind _sandstorm_8 (Variables|Default|GetSandStorm))
  (bind _sandstorm_9 (Variables|Default|GetSandStorm))
  (bind _sandstorm_10 (Variables|Default|GetSandStorm))
  (bind _sandstorm_11 (Variables|Default|GetSandStorm))
  (bind _sandstorm_12 (Variables|Default|GetSandStorm))
  (bind _sandstorm_13 (Variables|Default|GetSandStorm))
  (bind _sandstorm_14 (Variables|Default|GetSandStorm))
  (bind _sandstorm_15 (Variables|Default|GetSandStorm))
  (bind _sandstorm_16 (Variables|Default|GetSandStorm))
  (bind _sandstorm_17 (Variables|Default|GetSandStorm))
  (bind _particle_preview (Variables|Performance|GetParticle_Preview))
  (bind _sandstorm_18 (Variables|Default|GetSandStorm))
  (bind _sandstorm_19 (Variables|Default|GetSandStorm))
  (bind _sandstorm_20 (Variables|Default|GetSandStorm))
  (bind _sandstorm_21 (Variables|Default|GetSandStorm))
  (bind _sandstorm_22 (Variables|Default|GetSandStorm))
  (bind _returnvalue (Math|Conversions|ToVector(Float) _scale))
  ;[0.577 1 0 1 100] Set Niagara Parameters
  (Rendering|SetTranslucentSortPriority _sandstorm_16 (+ (Variables|/Script/Engine.PrimitiveComponent|GetTranslucencySortPriority _sandstorm_16) (Variables|Default|GetTranslucentSortPriority)))
  (Transformation|SetWorldScale3D (Variables|Default|GetDefaultSceneRoot) "1.000000,1.000000,1.000000")
  (Transformation|SetRelativeScale3D (Variables|Default|GetSandStorm) _returnvalue)
  (Transformation|SetRelativeScale3D (Variables|Default|GetControl_Rig) _returnvalue)
  (EventDispatchers|BindEventtoOnPreInitializeDelegate (Variables|Default|GetControlRig) (EventDispatchers|CreateEvent :!event BPSandStormAutoGenFunc))
  (switch Utilities|FlowControl|Switch|SwitchonSandStorm_Texture_Start (Variables|Default|GetStart_SmokeType)
    (:NewEnumerator0
      (Class|NiagaraComponent|SetVariableTexture _sandstorm_12 "Cm_A" "/Game/통합/Asset2/SandStorm/Textures/T_C_Cam06.T_C_Cam06")
      (Class|NiagaraComponent|SetVariableTexture _sandstorm_10 "Nm_A" "/Game/통합/Asset2/SandStorm/Textures/T_N_Cam06.T_N_Cam06")
      (Class|NiagaraComponent|SetVariableTexture _sandstorm_11 "Vm_A" "/Game/통합/Asset2/SandStorm/Textures/T_MV_Cam06.T_MV_Cam06"))
    (:NewEnumerator1
      (Class|NiagaraComponent|SetVariableTexture _sandstorm_12 "Cm_A" "/Game/통합/Asset2/SandStorm/Textures/T_C_Cam66.T_C_Cam66")
      (Class|NiagaraComponent|SetVariableTexture _sandstorm_10 "Nm_A" "/Game/통합/Asset2/SandStorm/Textures/T_N_Cam66.T_N_Cam66")
      (Class|NiagaraComponent|SetVariableTexture _sandstorm_11 "Vm_A" "/Game/통합/Asset2/SandStorm/Textures/T_MV_Cam66.T_MV_Cam66"))
    (:NewEnumerator2
      (Class|NiagaraComponent|SetVariableTexture _sandstorm_12 "Cm_A" "/Game/통합/Asset2/SandStorm/Textures/T_C_Cam666.T_C_Cam666")
      (Class|NiagaraComponent|SetVariableTexture _sandstorm_10 "Nm_A" "/Game/통합/Asset2/SandStorm/Textures/T_N_Cam666.T_N_Cam666")
      (Class|NiagaraComponent|SetVariableTexture _sandstorm_11 "Vm_A" "/Game/통합/Asset2/SandStorm/Textures/T_MV_Cam666.T_MV_Cam666")))
  (switch Utilities|FlowControl|Switch|SwitchonSandStorm_Texture_Middle (Variables|Default|GetMiddle_SmokeType)
    (:NewEnumerator0
      (Class|NiagaraComponent|SetVariableTexture _sandstorm_19 "Cm_B" "/Game/통합/Asset2/SandStorm/Textures/T_C_Cam02.T_C_Cam02")
      (Class|NiagaraComponent|SetVariableTexture _sandstorm_17 "Nm_B" "/Game/통합/Asset2/SandStorm/Textures/T_N_Cam02.T_N_Cam02")
      (Class|NiagaraComponent|SetVariableTexture _sandstorm_18 "Vm_B" "/Game/통합/Asset2/SandStorm/Textures/T_MV_Cam02.T_MV_Cam02"))
    (:NewEnumerator1
      (Class|NiagaraComponent|SetVariableTexture _sandstorm_19 "Cm_B" "/Game/통합/Asset2/SandStorm/Textures/T_C_Cam22.T_C_Cam22")
      (Class|NiagaraComponent|SetVariableTexture _sandstorm_17 "Nm_B" "/Game/통합/Asset2/SandStorm/Textures/T_N_Cam22.T_N_Cam22")
      (Class|NiagaraComponent|SetVariableTexture _sandstorm_18 "Vm_B" "/Game/통합/Asset2/SandStorm/Textures/T_MV_Cam22.T_MV_Cam22"))
    (:NewEnumerator2
      (Class|NiagaraComponent|SetVariableTexture _sandstorm_19 "Cm_B" "/Game/통합/Asset2/SandStorm/Textures/T_C_Cam222.T_C_Cam222")
      (Class|NiagaraComponent|SetVariableTexture _sandstorm_17 "Nm_B" "/Game/통합/Asset2/SandStorm/Textures/T_N_Cam222.T_N_Cam222")
      (Class|NiagaraComponent|SetVariableTexture _sandstorm_18 "Vm_B" "/Game/통합/Asset2/SandStorm/Textures/T_MV_Cam222.T_MV_Cam222"))
    (:NewEnumerator3
      (Class|NiagaraComponent|SetVariableTexture _sandstorm_15 "Cm_B" "/Game/통합/Asset2/SandStorm/Textures/T_C_Cam03.T_C_Cam03")
      (Class|NiagaraComponent|SetVariableTexture _sandstorm_13 "Nm_B" "/Game/통합/Asset2/SandStorm/Textures/T_N_Cam03.T_N_Cam03")
      (Class|NiagaraComponent|SetVariableTexture _sandstorm_14 "Vm_B" "/Game/통합/Asset2/SandStorm/Textures/T_MV_Cam03.T_MV_Cam03"))
    (:NewEnumerator4
      (Class|NiagaraComponent|SetVariableTexture _sandstorm_15 "Cm_B" "/Game/통합/Asset2/SandStorm/Textures/T_C_Cam33.T_C_Cam33")
      (Class|NiagaraComponent|SetVariableTexture _sandstorm_13 "Nm_B" "/Game/통합/Asset2/SandStorm/Textures/T_N_Cam33.T_N_Cam33")
      (Class|NiagaraComponent|SetVariableTexture _sandstorm_14 "Vm_B" "/Game/통합/Asset2/SandStorm/Textures/T_MV_Cam33.T_MV_Cam33"))
    (:NewEnumerator5
      (Class|NiagaraComponent|SetVariableTexture _sandstorm_15 "Cm_B" "/Game/통합/Asset2/SandStorm/Textures/T_C_Cam333.T_C_Cam333")
      (Class|NiagaraComponent|SetVariableTexture _sandstorm_13 "Nm_B" "/Game/통합/Asset2/SandStorm/Textures/T_N_Cam333.T_N_Cam333")
      (Class|NiagaraComponent|SetVariableTexture _sandstorm_14 "Vm_B" "/Game/통합/Asset2/SandStorm/Textures/T_MV_Cam333.T_MV_Cam333")))
  (switch Utilities|FlowControl|Switch|SwitchonSandStorm_Texture_End (Variables|Default|GetEnd_SmokeType)
    (:NewEnumerator0
      (Class|NiagaraComponent|SetVariableTexture _sandstorm_8 "Cm_C" "/Game/통합/Asset2/SandStorm/Textures/T_C_Cam02.T_C_Cam02")
      (Class|NiagaraComponent|SetVariableTexture _sandstorm_9 "Nm_C" "/Game/통합/Asset2/SandStorm/Textures/T_N_Cam02.T_N_Cam02")
      (Class|NiagaraComponent|SetVariableTexture _sandstorm_5 "Vm_C" "/Game/통합/Asset2/SandStorm/Textures/T_MV_Cam02.T_MV_Cam02"))
    (:NewEnumerator1
      (Class|NiagaraComponent|SetVariableTexture _sandstorm_8 "Cm_C" "/Game/통합/Asset2/SandStorm/Textures/T_C_Cam22.T_C_Cam22")
      (Class|NiagaraComponent|SetVariableTexture _sandstorm_9 "Nm_C" "/Game/통합/Asset2/SandStorm/Textures/T_N_Cam22.T_N_Cam22")
      (Class|NiagaraComponent|SetVariableTexture _sandstorm_5 "Vm_C" "/Game/통합/Asset2/SandStorm/Textures/T_MV_Cam22.T_MV_Cam22"))
    (:NewEnumerator2
      (Class|NiagaraComponent|SetVariableTexture _sandstorm_8 "Cm_C" "/Game/통합/Asset2/SandStorm/Textures/T_C_Cam222.T_C_Cam222")
      (Class|NiagaraComponent|SetVariableTexture _sandstorm_9 "Nm_C" "/Game/통합/Asset2/SandStorm/Textures/T_N_Cam222.T_N_Cam222")
      (Class|NiagaraComponent|SetVariableTexture _sandstorm_5 "Vm_C" "/Game/통합/Asset2/SandStorm/Textures/T_MV_Cam222.T_MV_Cam222"))
    (:NewEnumerator3
      (Class|NiagaraComponent|SetVariableTexture _sandstorm_22 "Cm_C" "/Game/통합/Asset2/SandStorm/Textures/T_C_Cam03.T_C_Cam03")
      (Class|NiagaraComponent|SetVariableTexture _sandstorm_20 "Nm_C" "/Game/통합/Asset2/SandStorm/Textures/T_N_Cam03.T_N_Cam03")
      (Class|NiagaraComponent|SetVariableTexture _sandstorm_21 "Vm_C" "/Game/통합/Asset2/SandStorm/Textures/T_MV_Cam03.T_MV_Cam03"))
    (:NewEnumerator4
      (Class|NiagaraComponent|SetVariableTexture _sandstorm_22 "Cm_C" "/Game/통합/Asset2/SandStorm/Textures/T_C_Cam33.T_C_Cam33")
      (Class|NiagaraComponent|SetVariableTexture _sandstorm_20 "Nm_C" "/Game/통합/Asset2/SandStorm/Textures/T_N_Cam33.T_N_Cam33")
      (Class|NiagaraComponent|SetVariableTexture _sandstorm_21 "Vm_C" "/Game/통합/Asset2/SandStorm/Textures/T_MV_Cam33.T_MV_Cam33"))
    (:NewEnumerator5
      (Class|NiagaraComponent|SetVariableTexture _sandstorm_22 "Cm_C" "/Game/통합/Asset2/SandStorm/Textures/T_C_Cam333.T_C_Cam333")
      (Class|NiagaraComponent|SetVariableTexture _sandstorm_20 "Nm_C" "/Game/통합/Asset2/SandStorm/Textures/T_N_Cam333.T_N_Cam333")
      (Class|NiagaraComponent|SetVariableTexture _sandstorm_21 "Vm_C" "/Game/통합/Asset2/SandStorm/Textures/T_MV_Cam333.T_MV_Cam333")))
  (Utilities|FlowControl|Sequence
    (:then_0
      (Class|NiagaraComponent|SetVariableInt _sandstorm_7 "visibility" (Math|Conversions|ToInteger(Boolean) (not _particle_preview)))
      (Class|NiagaraComponent|SetVariableInt _sandstorm_7 "visibility02" (Math|Conversions|ToInteger(Boolean) _particle_preview))
      (Niagara|SetNiagaraVariable(Float) _sandstorm_7 "Spawn Rate" (Variables|Performance|GetSpawn%20Rate))
      (Niagara|SetNiagaraVariable(Float) _sandstorm_7 "KillChance_Start" (Variables|Performance|GetKillChance_Start))
      (Niagara|SetNiagaraVariable(Float) _sandstorm_7 "KillChance_Middle" (Variables|Performance|GetKillChance_Middle))
      (Niagara|SetNiagaraVariable(Float) _sandstorm_7 "KillChance_End" (Variables|Performance|GetKillChance_End))
      (Niagara|SetNiagaraVariable(Float) _sandstorm_4 "ScaleSize" (* (Variables|Performance|GetScaleSize_All) (Variables|Basic|GetScale)))
      (Niagara|SetNiagaraVariable(Float) _sandstorm_4 "MinScale" (Variables|Performance|GetMinScale_All))
      (Niagara|SetNiagaraVariable(Float) _sandstorm_4 "maxScale" (Variables|Performance|GetMaxScale_All))
      (Niagara|SetNiagaraVariable(LinearColor) _sandstorm "TintColor_Start" (Variables|Color|GetTintColor_Start))
      (Niagara|SetNiagaraVariable(LinearColor) _sandstorm "TintColor_Middle" (Variables|Color|GetTintColor_Middle))
      (Niagara|SetNiagaraVariable(LinearColor) _sandstorm "TintColor_End" (Variables|Color|GetTintColor_End))
      (Niagara|SetNiagaraVariable(LinearColor) _sandstorm "ColorArea_A" (Variables|Color|GetColorArea_A))
      (Niagara|SetNiagaraVariable(LinearColor) _sandstorm "ColorArea_B" (Variables|Color|GetColorArea_B))
      (Niagara|SetNiagaraVariable(LinearColor) _sandstorm "ColorArea_C" (Variables|Color|GetColorArea_C))
      (Niagara|SetNiagaraVariable(Float) (Variables|Default|GetSandStorm) "NormalScale" (Variables|Color|GetNormalScale))
      (Niagara|SetNiagaraVariable(Float) _sandstorm_3 "Contrast_Start" (Variables|Color|GetContrast_Start))
      (Niagara|SetNiagaraVariable(Float) _sandstorm_3 "Contrast_Middle" (Variables|Color|GetContrast_Middle))
      (Niagara|SetNiagaraVariable(Float) _sandstorm_3 "Contrast_End" (Variables|Color|GetContrast_End))
      (Niagara|SetNiagaraVariable(Float) _sandstorm_2 "Lifetime_Scale" (Variables|Time|GetLifetime_Scale))
      (Niagara|SetNiagaraVariable(Float) _sandstorm_2 "Loop Duration" (Variables|Time|GetLoop%20Duration))
      (Niagara|SetNiagaraVariable(Float) _sandstorm_6 "RotationRate_Scale" (Variables|Movement|GetRotationRate_Scale))
      (Niagara|SetNiagaraVariable(Float) _sandstorm_6 "Velocity Speed Scale" (Variables|Movement|GetVelocity%20Speed%20Scale))
      (Niagara|SetNiagaraVariable(Float) _sandstorm_6 "WavePeriod" (Variables|Movement|GetWavePeriod))
      (Niagara|SetNiagaraVariable(Float) _sandstorm_6 "WaveScale" (Variables|Movement|GetWaveScale))
      (Niagara|SetNiagaraVariable(Float) _sandstorm_6 "Bound" (Variables|Basic|GetScale))
      (Niagara|SetNiagaraVariable(Float) _sandstorm_6 "SandNoiseA" (Variables|SandNoise|GetSandNoiseA))
      (Niagara|SetNiagaraVariable(Float) _sandstorm_6 "SandNoiseB" (Variables|SandNoise|GetSandNoiseB))
      (Niagara|SetNiagaraVariable(Float) _sandstorm_6 "SandNoiseC" (Variables|SandNoise|GetSandNoiseC))
      (Niagara|SetNiagaraVariable(Float) _sandstorm_6 "SandNoiseScale" (Variables|SandNoise|GetSandNoiseScale))
      (Niagara|SetNiagaraVariable(Float) _sandstorm_6 "FadeDistance" (Variables|Color|GetFadeDistance))
      (Niagara|SetNiagaraVariable(Float) _sandstorm_6 "Emessive" (Variables|Color|GetEmessive))
      (Niagara|SetNiagaraVariable(Float) _sandstorm_6 "Scale_Start" (Variables|Performance|GetScaleSize_Start))
      (Niagara|SetNiagaraVariable(Float) _sandstorm_6 "Scale_Middle" (Variables|Performance|GetScaleSize_Middle))
      (Niagara|SetNiagaraVariable(Float) _sandstorm_6 "Scale_End" (Variables|Performance|GetScaleSize_End)))
    (:then_1
      (Rendering|SetVisibility (Variables|Default|GetSkeletalMesh) (Variables|Basic|GetMeshPreview) false))))

(fn BPSandStormAutoGenFunc
  (params (Component :type Control%20Rig%20Component%20Object%20Reference))
  (Class|ControlRigComponent|AddMappedCompleteSkeletalMesh Component (Variables|Default|GetSkeletalMesh))
  (Class|ControlRigComponent|AddMappedComponents Component (Utilities|Array|MakeArray (Utilities|Struct|MakeControlRigComponentMappedComponent (Variables|Default|GetGuide_01) "point_0_ctrl" "Control" "Input") (Utilities|Struct|MakeControlRigComponentMappedComponent (Variables|Default|GetGuide_02) "point_2_ctrl" "Control" "Input") (Utilities|Struct|MakeControlRigComponentMappedComponent (Variables|Default|GetGuide_03) "point_4_ctrl" "Control" "Input") (Utilities|Struct|MakeControlRigComponentMappedComponent (Variables|Default|GetGuide_04) "point_6_ctrl" "Control" "Input") (Utilities|Struct|MakeControlRigComponentMappedComponent (Variables|Default|GetGuide_05) "point_8_ctrl" "Control" "Input"))))