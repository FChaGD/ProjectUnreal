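; BP_Tornado is a configurable sandstorm tornado effect built from skeletal mesh layers and Niagara systems, set up entirely in the construction script.
; Height drives dynamic material opacity, color and shape, and fades in particle spawn rates near its upper range.
; Scale resizes the actor and particles, while other variables tune color, tiling, speed and sort priority.
; Two Control Rigs deform the funnel meshes from guide components, allowing the tornado to bend.
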(event EventBeginPlay)

(event Collision|EventActorBeginOverlap
  (params (OtherActor :type Actor%20Object%20Reference)))

(event EventTick
  (params (DeltaSeconds :type Float%20%28single-precision%29)))

(fn ConstructionScript
  (bind _height (Variables|Basic|GetHeight))
  (bind _speedtime_uptornadoa (Variables|Default|GetSpeedTime_UPTornadoA))
  (bind _speedtime_uptornadob (Variables|Default|GetSpeedTime_UPTornadoB))
  (bind _speedtime_side (Variables|Default|GetSpeedTime_Side))
  (bind _speedtime_core_ (Variables|Default|GetSpeedTime_Core_))
  (bind _speedtime_core (Variables|Core|GetSpeedTime_Core))
  (bind _speedtime (Variables|Basic|GetSpeedTime))
  (bind _speedtime_2 (Variables|Basic|GetSpeedTime))
  (bind _speedtime_3 (Variables|Basic|GetSpeedTime))
  (bind _speedalongy_uptornadoa (Variables|Default|GetSpeedAlongY_UPTornadoA))
  (bind _speedalongy_uptornadob (Variables|Default|GetSpeedAlongY_UPTornadoB))
  (bind _speedalongy_side (Variables|Default|GetSpeedAlongY_Side))
  (bind _speedalongy_core (Variables|Default|GetSpeedAlongY_Core))
  (bind _speedtime_core_2 (Variables|Core|GetSpeedTime_Core))
  (bind _speedtime_4 (Variables|Basic|GetSpeedTime))
  (bind _speedtime_5 (Variables|Basic|GetSpeedTime))
  (bind _speedtime_6 (Variables|Basic|GetSpeedTime))
  (bind _tornado_mesh (Variables|Default|GetTornado_mesh))
  (bind _tornado (Variables|Default|GetTornado))
  (bind _tornado_mesh_2 (Variables|Default|GetTornado_mesh))
  (bind _tornado_2 (Variables|Default|GetTornado))
  (bind _color_alpha (Variables|Basic|GetColor_Alpha))
  (bind _core (Variables|Default|GetCore))
  (bind _skm_sidetornado (Variables|Default|GetSKM_SideTornado))
  (bind _tornado_3 (Variables|Default|GetTornado))
  (bind _skm_uptornadoa (Variables|Default|GetSKM_UPTornadoA))
  (bind _skm_uptornadob (Variables|Default|GetSKM_UPTornadoB))
  (bind _tornado_mesh_3 (Variables|Default|GetTornado_mesh))
  (bind _tornado_mesh_4 (Variables|Default|GetTornado_mesh))
  (bind _tornado_mesh_5 (Variables|Default|GetTornado_mesh))
  (bind _height_2 (Variables|Basic|GetHeight))
  (bind _sidetornado (Variables|Default|GetSideTornado))
  (bind _sidetornado_2 (Variables|Default|GetSideTornado))
  (bind _sidetornado_3 (Variables|Default|GetSideTornado))
  (bind _poweralpha_uptornadoa (Variables|Default|GetPowerAlpha_UPTornadoA))
  (bind _poweralpha_uptornadob (Variables|Default|GetPowerAlpha_UPTornadoB))
  (bind _poweralpha_side (Variables|Default|GetPowerAlpha_Side))
  (bind _poweralpha_core (Variables|Default|GetPowerAlpha_Core))
  (bind _dotpower_uptornadoa (Variables|Default|GetDotPower_UPTornadoA))
  (bind _dotpower_uptornadob (Variables|Default|GetDotPower_UPTornadoB))
  (bind _dotpower_side (Variables|Default|GetDotPower_Side))
  (bind _dotpower_core (Variables|Default|GetDotPower_Core))
  (bind _tile_uptornadoa (Variables|Default|GetTile_UPTornadoA))
  (bind _tile_uptornadob (Variables|Default|GetTile_UPTornadoB))
  (bind _tile_side (Variables|Default|GetTile_Side))
  (bind _tile_core (Variables|Default|GetTile_Core))
  (bind (_x _y) (Math|Vector2D|BreakVector2D _tile_uptornadoa))
  (bind (_x_2 _y_2) (Math|Vector2D|BreakVector2D _tile_uptornadob))
  (bind (_x_3 _y_3) (Math|Vector2D|BreakVector2D _tile_side))
  (bind (_x_4 _y_4) (Math|Vector2D|BreakVector2D _tile_core))
  (bind _returnvalue (* _speedtime_uptornadoa _speedtime_3))
  (bind _returnvalue_2 (* _speedtime_uptornadob _speedtime_2))
  (bind _returnvalue_3 (* _speedtime_side _speedtime))
  (bind _returnvalue_4 (* _speedtime_core_ _speedtime_core))
  (bind _returnvalue_5 (* _speedalongy_uptornadoa _speedtime_6))
  (bind _returnvalue_6 (* _speedalongy_uptornadob _speedtime_5))
  (bind _returnvalue_7 (* _speedalongy_side _speedtime_4))
  (bind _returnvalue_8 (* _speedalongy_core _speedtime_core_2))
  (EventDispatchers|BindEventtoOnPreInitializeDelegate (Variables|Default|GetControlRig) (EventDispatchers|CreateEvent :!event BPTornadoAutoGenFunc1))
  (EventDispatchers|BindEventtoOnPreInitializeDelegate (Variables|Default|GetControlRig1) (EventDispatchers|CreateEvent :!event BPTornadoAutoGenFunc))
  ;[0 0.1579 1 1 100] Set Translucent Sort priority
  (Rendering|SetTranslucentSortPriority _tornado_mesh_5 (+ (Variables|/Script/Engine.PrimitiveComponent|GetTranslucencySortPriority _tornado_mesh_5) (Variables|Basic|GetTranslucentSortPriority)))
  (Rendering|SetTranslucentSortPriority _sidetornado_3 (+ (Variables|/Script/Engine.PrimitiveComponent|GetTranslucencySortPriority _sidetornado_3) (Variables|Basic|GetTranslucentSortPriority)))
  (Rendering|SetTranslucentSortPriority _core (+ (Variables|/Script/Engine.PrimitiveComponent|GetTranslucencySortPriority _core) (Variables|Basic|GetTranslucentSortPriority)))
  (Rendering|SetTranslucentSortPriority _skm_sidetornado (+ (Variables|/Script/Engine.PrimitiveComponent|GetTranslucencySortPriority _skm_sidetornado) (Variables|Basic|GetTranslucentSortPriority)))
  (Rendering|SetTranslucentSortPriority _tornado_3 (+ (Variables|/Script/Engine.PrimitiveComponent|GetTranslucencySortPriority _tornado_3) (Variables|Basic|GetTranslucentSortPriority)))
  (Rendering|SetTranslucentSortPriority _skm_uptornadoa (+ (Variables|/Script/Engine.PrimitiveComponent|GetTranslucencySortPriority _skm_uptornadoa) (Variables|Basic|GetTranslucentSortPriority)))
  (Rendering|SetTranslucentSortPriority _skm_uptornadob (+ (Variables|/Script/Engine.PrimitiveComponent|GetTranslucencySortPriority _skm_uptornadob) (Variables|Basic|GetTranslucentSortPriority)))
  ;[0 0.8192 1 1 100] Set Scale
  (Transformation|SetWorldScale3D (Variables|Default|GetDefaultSceneRoot) (Math|Conversions|ToVector(Float) (/ (Variables|Basic|GetScale) 1e+02)))
  (Utilities|FlowControl|Sequence
    (:then_0
      ;[0 1 0.316 1 100] Set Material
      (bind _returnvalue_9 (Rendering|Material|CreateDynamicMaterialInstance (Variables|Default|GetSKM_UPTornadoA) 0 "/Game/통합/Asset2/SandStorm/Materials/MI_Tornado_Inst2.MI_Tornado_Inst2" "None" :!class /Script/Engine.PrimitiveComponent))
      (Variables|Default|SetUpAMat _returnvalue_9)
      (bind _returnvalue_10 (Rendering|Material|CreateDynamicMaterialInstance (Variables|Default|GetSKM_UPTornadoB) 0 "/Game/통합/Asset2/SandStorm/Materials/MI_Tornado_Inst3.MI_Tornado_Inst3" "None" :!class /Script/Engine.PrimitiveComponent))
      (Variables|Default|SetUpBMat _returnvalue_10)
      (bind _returnvalue_11 (Rendering|Material|CreateDynamicMaterialInstance (Variables|Default|GetCore) 0 "/Game/통합/Asset2/SandStorm/Materials/MI_Tornado_Inst.MI_Tornado_Inst" "None" :!class /Script/Engine.PrimitiveComponent))
      (Variables|Default|SetCoreMat _returnvalue_11)
      (bind _returnvalue_12 (Rendering|Material|CreateDynamicMaterialInstance (Variables|Default|GetSKM_SideTornado) 0 "/Game/통합/Asset2/SandStorm/Materials/MI_Tornado_Inst1.MI_Tornado_Inst1" "None" :!class /Script/Engine.PrimitiveComponent))
      (Variables|Default|SetSideMat _returnvalue_12)
      ;[0.6736 1 0.02728 1 100] Change niagara location
      (Transformation|SetRelativeLocation (Variables|Default|GetTornado) (Math|Vector|MakeVector 0.0 0.0 (Math|Float|MapRangeClamped _height_2 8e+01 1e+02 (* (.Z (Math|Vector|BreakVector (Variables|/Script/Engine.SceneComponent|GetRelativeLocation (Variables|Default|GetA)))) (Math|Curves|GetFloatValue (Variables|Default|GetHeightCurve) (Math|Float|MapRangeClamped _height_2 8e+01 1e+02 0.0 1.0))) 0.0)) false false)
      ;[1 0.3154 0 1 100] Set Material Parameters
      (Rendering|Material|SetScalarParameterValue (Variables|Default|GetCoreMat) "AlphaVertex" (Math|Float|MapRangeClamped (Variables|Basic|GetHeight) 0.0 1e+02 8e+01 -1.0) :!class /Script/Engine.MaterialInstanceDynamic)
      (Rendering|Material|SetScalarParameterValue (Variables|Default|GetUpBMat) "AlphaVertex" (Math|Float|MapRangeClamped _height 0.0 9e+01 2e+02 -1.0) :!class /Script/Engine.MaterialInstanceDynamic)
      (Rendering|Material|SetScalarParameterValue (Variables|Default|GetUpAMat) "AlphaVertex" (Math|Float|MapRangeClamped _height 0.0 9e+01 2e+02 -1.0) :!class /Script/Engine.MaterialInstanceDynamic)
      (Rendering|Material|SetScalarParameterValue (Variables|Default|GetUpAMat) "Alpha" (Math|Float|MapRangeClamped (Variables|Basic|GetHeight) 0.0 1e+02 0.0 (Variables|Default|GetAlpha_UPTornadoA)) :!class /Script/Engine.MaterialInstanceDynamic)
      (Rendering|Material|SetScalarParameterValue (Variables|Default|GetUpBMat) "Alpha" (Math|Float|MapRangeClamped (Variables|Basic|GetHeight) 0.0 1e+02 0.0 (Variables|Default|GetAlpha_UPTornadoB)) :!class /Script/Engine.MaterialInstanceDynamic)
      (Rendering|Material|SetScalarParameterValue (Variables|Default|GetSideMat) "Alpha" (Math|Float|MapRangeClamped (Variables|Basic|GetHeight) 0.0 1e+02 0.0 (Variables|Default|GetAlpha_Side)) :!class /Script/Engine.MaterialInstanceDynamic)
      (Rendering|Material|SetScalarParameterValue (Variables|Default|GetCoreMat) "Alpha" (Math|Float|MapRangeClamped (Variables|Basic|GetHeight) 0.0 1e+02 0.0 (Variables|Default|GetAlpha_Core)) :!class /Script/Engine.MaterialInstanceDynamic)
      (Rendering|Material|SetScalarParameterValue (Variables|Default|GetUpAMat) "PowerAlpha" (Math|Float|MapRangeClamped (Variables|Basic|GetHeight) 0.0 1e+02 (* _poweralpha_uptornadoa (Variables|Default|GetPowerMulty)) (* _poweralpha_uptornadoa (Variables|Basic|GetContrast))) :!class /Script/Engine.MaterialInstanceDynamic)
      (Rendering|Material|SetScalarParameterValue (Variables|Default|GetUpBMat) "PowerAlpha" (Math|Float|MapRangeClamped (Variables|Basic|GetHeight) 0.0 1e+02 (* _poweralpha_uptornadob (Variables|Default|GetPowerMulty)) (* _poweralpha_uptornadob (Variables|Basic|GetContrast))) :!class /Script/Engine.MaterialInstanceDynamic)
      (Rendering|Material|SetScalarParameterValue (Variables|Default|GetSideMat) "PowerAlpha" (Math|Float|MapRangeClamped (Variables|Basic|GetHeight) 0.0 1e+02 (* _poweralpha_side (Variables|Default|GetPowerMulty)) (* _poweralpha_side (Variables|Core|GetContrast_Core))) :!class /Script/Engine.MaterialInstanceDynamic)
      (Rendering|Material|SetScalarParameterValue (Variables|Default|GetCoreMat) "PowerAlpha" (Math|Float|MapRangeClamped (Variables|Basic|GetHeight) 0.0 1e+02 (* _poweralpha_core (Variables|Default|GetPowerMulty)) (* _poweralpha_core (Variables|Core|GetContrast_Core))) :!class /Script/Engine.MaterialInstanceDynamic)
      (Rendering|Material|SetVectorParameterValue (Variables|Default|GetCoreMat) "Color_A" (Math|Color|Lerp(LinearColor) "(R=1.000000,G=1.000000,B=1.000000,A=1.000000)" (Variables|Basic|GetColor_Alpha) (Math|Float|MapRangeClamped (Variables|Basic|GetHeight) 0.0 1e+02 0.0 1.0)) :!class /Script/Engine.MaterialInstanceDynamic)
      (Rendering|Material|SetVectorParameterValue (Variables|Default|GetSideMat) "Color_A" (Math|Color|Lerp(LinearColor) "(R=1.000000,G=1.000000,B=1.000000,A=1.000000)" (Variables|Basic|GetColor_Alpha) (Math|Float|MapRangeClamped (Variables|Basic|GetHeight) 0.0 1e+02 0.0 1.0)) :!class /Script/Engine.MaterialInstanceDynamic)
      (Rendering|Material|SetVectorParameterValue (Variables|Default|GetUpAMat) "Color_A" (Math|Color|Lerp(LinearColor) "(R=1.000000,G=1.000000,B=1.000000,A=1.000000)" (Variables|Basic|GetColor_Alpha) (Math|Float|MapRangeClamped (Variables|Basic|GetHeight) 0.0 1e+02 0.0 1.0)) :!class /Script/Engine.MaterialInstanceDynamic)
      (Rendering|Material|SetVectorParameterValue (Variables|Default|GetUpBMat) "Color_A" (Math|Color|Lerp(LinearColor) "(R=1.000000,G=1.000000,B=1.000000,A=1.000000)" (Variables|Basic|GetColor_Alpha) (Math|Float|MapRangeClamped (Variables|Basic|GetHeight) 0.0 1e+02 0.0 1.0)) :!class /Script/Engine.MaterialInstanceDynamic)
      (Rendering|Material|SetScalarParameterValue (Variables|Default|GetUpAMat) "TileX" (+ _x (/ (Variables|Basic|GetTileWidth) 1e+02)) :!class /Script/Engine.MaterialInstanceDynamic)
      (Rendering|Material|SetScalarParameterValue (Variables|Default|GetUpAMat) "TileY" (+ _y (/ (Variables|Basic|GetTileHeight) 1e+02)) :!class /Script/Engine.MaterialInstanceDynamic)
      (Rendering|Material|SetScalarParameterValue (Variables|Default|GetUpBMat) "TileX" (+ _x_2 (/ (Variables|Basic|GetTileWidth) 1e+02)) :!class /Script/Engine.MaterialInstanceDynamic)
      (Rendering|Material|SetScalarParameterValue (Variables|Default|GetUpBMat) "TileY" (+ (/ (Variables|Basic|GetTileHeight) 1e+02) _y_2) :!class /Script/Engine.MaterialInstanceDynamic)
      (Rendering|Material|SetScalarParameterValue (Variables|Default|GetSideMat) "TileX" (+ _x_3 (/ (Variables|Core|GetTileWidth_Core) 1e+02)) :!class /Script/Engine.MaterialInstanceDynamic)
      (Rendering|Material|SetScalarParameterValue (Variables|Default|GetSideMat) "TileY" (+ _y_3 (/ (Variables|Core|GetTileHeight_Core) 1e+02)) :!class /Script/Engine.MaterialInstanceDynamic)
      (Rendering|Material|SetScalarParameterValue (Variables|Default|GetCoreMat) "TileX" (+ _x_4 (/ (Variables|Core|GetTileWidth_Core) 1e+02)) :!class /Script/Engine.MaterialInstanceDynamic)
      (Rendering|Material|SetScalarParameterValue (Variables|Default|GetCoreMat) "TileY" (+ _y_4 (/ (Variables|Core|GetTileHeight_Core) 1e+02)) :!class /Script/Engine.MaterialInstanceDynamic)
      (Rendering|Material|SetScalarParameterValue (Variables|Default|GetUpAMat) "DotPower" (Math|Float|MapRangeClamped (Variables|Basic|GetHeight) 0.0 1e+02 (* _dotpower_uptornadoa (Variables|Default|GetDotPowerMulty)) (* _dotpower_uptornadoa (Variables|Basic|GetEdgePower))) :!class /Script/Engine.MaterialInstanceDynamic)
      (Rendering|Material|SetScalarParameterValue (Variables|Default|GetUpBMat) "DotPower" (Math|Float|MapRangeClamped (Variables|Basic|GetHeight) 0.0 1e+02 (* _dotpower_uptornadob (Variables|Default|GetDotPowerMulty)) (* _dotpower_uptornadob (Variables|Basic|GetEdgePower))) :!class /Script/Engine.MaterialInstanceDynamic)
      (Rendering|Material|SetScalarParameterValue (Variables|Default|GetSideMat) "DotPower" (Math|Float|MapRangeClamped (Variables|Basic|GetHeight) 0.0 1e+02 (* _dotpower_side (Variables|Default|GetDotPowerMulty)) (* _dotpower_side (Variables|Basic|GetEdgePower))) :!class /Script/Engine.MaterialInstanceDynamic)
      (Rendering|Material|SetScalarParameterValue (Variables|Default|GetCoreMat) "DotPower" (Math|Float|MapRangeClamped (Variables|Basic|GetHeight) 0.0 1e+02 (* _dotpower_core (Variables|Default|GetDotPowerMulty)) (* _dotpower_core (Variables|Basic|GetEdgePower))) :!class /Script/Engine.MaterialInstanceDynamic)
      (Rendering|Material|SetScalarParameterValue (Variables|Default|GetUpAMat) "SpeedTime" (Math|Float|MapRangeClamped (Variables|Basic|GetHeight) 0.0 1e+02 _returnvalue _returnvalue) :!class /Script/Engine.MaterialInstanceDynamic)
      (Rendering|Material|SetScalarParameterValue (Variables|Default|GetUpBMat) "SpeedTime" (Math|Float|MapRangeClamped (Variables|Basic|GetHeight) 0.0 1e+02 _returnvalue_2 _returnvalue_2) :!class /Script/Engine.MaterialInstanceDynamic)
      (Rendering|Material|SetScalarParameterValue (Variables|Default|GetSideMat) "SpeedTime" (Math|Float|MapRangeClamped (Variables|Basic|GetHeight) 0.0 1e+02 _returnvalue_3 _returnvalue_3) :!class /Script/Engine.MaterialInstanceDynamic)
      (Rendering|Material|SetScalarParameterValue (Variables|Default|GetCoreMat) "SpeedTime" (Math|Float|MapRangeClamped (Variables|Basic|GetHeight) 0.0 1e+02 _returnvalue_4 _returnvalue_4) :!class /Script/Engine.MaterialInstanceDynamic)
      (Rendering|Material|SetScalarParameterValue (Variables|Default|GetUpAMat) "SpeedAlongY" (Math|Float|MapRangeClamped (Variables|Basic|GetHeight) 0.0 1e+02 _returnvalue_5 _returnvalue_5) :!class /Script/Engine.MaterialInstanceDynamic)
      (Rendering|Material|SetScalarParameterValue (Variables|Default|GetUpBMat) "SpeedAlongY" (Math|Float|MapRangeClamped (Variables|Basic|GetHeight) 0.0 1e+02 _returnvalue_6 _returnvalue_6) :!class /Script/Engine.MaterialInstanceDynamic)
      (Rendering|Material|SetScalarParameterValue (Variables|Default|GetSideMat) "SpeedAlongY" (Math|Float|MapRangeClamped (Variables|Basic|GetHeight) 0.0 1e+02 _returnvalue_7 _returnvalue_7) :!class /Script/Engine.MaterialInstanceDynamic)
      (Rendering|Material|SetScalarParameterValue (Variables|Default|GetCoreMat) "SpeedAlongY" (Math|Float|MapRangeClamped (Variables|Basic|GetHeight) 0.0 1e+02 _returnvalue_8 _returnvalue_8) :!class /Script/Engine.MaterialInstanceDynamic)
      (Rendering|Material|SetScalarParameterValue (Variables|Default|GetUpAMat) "Emessive" (Math|Float|MapRangeClamped (Variables|Basic|GetHeight) 0.0 1e+02 0.0 (* (Variables|Default|GetEmessiveAll) (Variables|Basic|GetEmessive))) :!class /Script/Engine.MaterialInstanceDynamic)
      (Rendering|Material|SetScalarParameterValue (Variables|Default|GetUpBMat) "Emessive" (Math|Float|MapRangeClamped (Variables|Basic|GetHeight) 0.0 1e+02 0.0 (* (Variables|Default|GetEmessiveAll) (Variables|Basic|GetEmessive))) :!class /Script/Engine.MaterialInstanceDynamic)
      (Rendering|Material|SetScalarParameterValue (Variables|Default|GetSideMat) "Emessive" (Math|Float|MapRangeClamped (Variables|Basic|GetHeight) 0.0 1e+02 0.0 (* (Variables|Default|GetEmessiveAll) (Variables|Basic|GetEmessive))) :!class /Script/Engine.MaterialInstanceDynamic)
      (Rendering|Material|SetScalarParameterValue (Variables|Default|GetCoreMat) "Emessive" (Math|Float|MapRangeClamped (Variables|Basic|GetHeight) 0.0 1e+02 0.0 (* (Variables|Default|GetEmessiveAll) (Variables|Basic|GetEmessive))) :!class /Script/Engine.MaterialInstanceDynamic)
      (Rendering|Material|SetScalarParameterValue (Variables|Default|GetUpAMat) "NormalMap" (Math|Float|MapRangeClamped (Variables|Basic|GetHeight) 0.0 1e+02 0.0 (* (Variables|Default|GetNormalMapAll) (Variables|Basic|GetNormalMap_Intensity))) :!class /Script/Engine.MaterialInstanceDynamic)
      (Rendering|Material|SetScalarParameterValue (Variables|Default|GetUpBMat) "NormalMap" (Math|Float|MapRangeClamped (Variables|Basic|GetHeight) 0.0 1e+02 0.0 (* (Variables|Default|GetNormalMapAll) (Variables|Basic|GetNormalMap_Intensity))) :!class /Script/Engine.MaterialInstanceDynamic)
      (Rendering|Material|SetScalarParameterValue (Variables|Default|GetSideMat) "NormalMap" (Math|Float|MapRangeClamped (Variables|Basic|GetHeight) 0.0 1e+02 0.0 (* (Variables|Default|GetNormalMapAll) (Variables|Basic|GetNormalMap_Intensity))) :!class /Script/Engine.MaterialInstanceDynamic)
      (Rendering|Material|SetScalarParameterValue (Variables|Default|GetCoreMat) "NormalMap" (Math|Float|MapRangeClamped (Variables|Basic|GetHeight) 0.0 1e+02 0.0 (* (Variables|Default|GetNormalMapAll) (Variables|Basic|GetNormalMap_Intensity))) :!class /Script/Engine.MaterialInstanceDynamic))
    (:then_1
      ;[0.2066 0 1 1 100] Set Niagara Parameters
      (Niagara|SetNiagaraVariable(Float) (Variables|Default|GetTornado) "Smoke_SpawnRate_Scale" (* (Variables|Particles|GetSmoke_SpawnRate_Scale) (Math|Float|MapRangeClamped (Variables|Basic|GetHeight) 8e+01 85.0 0.0 1.0)))
      (Niagara|SetNiagaraVariable(Float) _tornado_mesh_4 "Particle_SpawnRate_Scale" (* (Variables|Particles|GetParticle_SpawnRate_Scale) (Math|Float|MapRangeClamped (Variables|Basic|GetHeight) 8e+01 85.0 0.0 1.0)))
      (Niagara|SetNiagaraVariable(Float) _tornado_mesh_4 "Mesh_SpawnRate_Scale" (* (Variables|Particles|GetMesh_SpawnRate_Scale) (Math|Float|MapRangeClamped (Variables|Basic|GetHeight) 8e+01 85.0 0.0 1.0)))
      (Niagara|SetNiagaraVariable(LinearColor) _tornado "Smoke_Color_A" (Variables|Particles|GetSmoke_Color_A))
      (Niagara|SetNiagaraVariable(LinearColor) _tornado "Smoke_Color_B" (Variables|Particles|GetSmoke_Color_B))
      (Niagara|SetNiagaraVariable(LinearColor) _tornado_mesh_2 "Particle_Color_A" (Variables|Particles|GetParticle_Color_A))
      (Niagara|SetNiagaraVariable(LinearColor) _tornado_mesh_2 "Particle_Color_B" (Variables|Particles|GetParticle_Color_B))
      (Niagara|SetNiagaraVariable(LinearColor) _tornado_mesh "Mesh_Color_A" (Variables|Particles|GetMesh_Color_A))
      (Niagara|SetNiagaraVariable(LinearColor) _tornado_mesh "Mesh_Color_B" (Variables|Particles|GetMesh_Color_B))
      (Niagara|SetNiagaraVariable(Float) (Variables|Default|GetTornado) "Emessive_Scale" (Variables|Particles|GetEmessive_Scale))
      (Niagara|SetNiagaraVariable(Float) (Variables|Default|GetTornado) "Contrast_Scale" (Variables|Particles|GetContrast_Scale))
      (Niagara|SetNiagaraVariable(Float) (Variables|Default|GetTornado) "Smoke_Size_Scale" (* (Variables|Particles|GetSmoke_Size_Scale) (/ (Variables|Basic|GetScale) 1e+02)))
      (Niagara|SetNiagaraVariable(Float) _tornado_mesh_3 "particle_Size_Scale" (* (Variables|Particles|Getparticle_Size_Scale) (/ (Variables|Basic|GetScale) 1e+02)))
      (Niagara|SetNiagaraVariable(Float) _tornado_mesh_3 "Mesh _Scale" (* (Variables|Particles|GetMesh%20_Scale) (Math|Curves|GetFloatValue (Variables|Default|GetScaleCurve) (Variables|Basic|GetScale))))
      (Niagara|SetNiagaraVariable(Float) _tornado_mesh_3 "Mesh_Scale_2" (* (Variables|Particles|GetMesh%20_Scale_2) (Math|Curves|GetFloatValue (Variables|Default|GetScaleCurve) (Variables|Basic|GetScale))))
      (Niagara|SetNiagaraVariable(Float) _sidetornado "SpawnRate" (* (Variables|Particles|GetSmoke_SpawnRate_Scale) (Math|Float|MapRangeClamped (Variables|Basic|GetHeight) 8e+01 85.0 0.0 1.0)))
      (Niagara|SetNiagaraVariable(Float) _sidetornado "Smoke_Scale_Size" (* (Variables|Particles|GetSmoke_Size_Scale) (/ (Variables|Basic|GetScale) 1e+02)))
      (Niagara|SetNiagaraVariable(Float) _sidetornado "Emessive" (Variables|Basic|GetEmessive))
      (Niagara|SetNiagaraVariable(Float) _sidetornado "Contrast_Scale" (Variables|Particles|GetContrast_Scale))
      (Niagara|SetNiagaraVariable(LinearColor) _sidetornado "Smoke_Color_A" _color_alpha)
      (Niagara|SetNiagaraVariable(LinearColor) _sidetornado "Smoke_Color_B" _color_alpha)
      (Niagara|SetNiagaraVariable(Float) _sidetornado_2 "SandLerp" (Variables|Particles|GetSandLerp))
      (Niagara|SetNiagaraVariable(Float) _sidetornado_2 "SandNoiseScale" (Variables|Particles|GetSandNoiseScale))
      (Niagara|SetNiagaraVariable(Float) _tornado_2 "SandLerp" (Variables|Particles|GetSandLerp))
      (Niagara|SetNiagaraVariable(Float) _tornado_2 "SandNoiseScale" (Variables|Particles|GetSandNoiseScale)))))

(fn BPTornadoAutoGenFunc1
  (params (Component :type Control%20Rig%20Component%20Object%20Reference))
  (Class|ControlRigComponent|AddMappedCompleteSkeletalMesh Component (Variables|Default|GetCore))
  (Class|ControlRigComponent|AddMappedCompleteSkeletalMesh Component (Variables|Default|GetSKM_SideTornado))
  (Class|ControlRigComponent|AddMappedComponents Component (Utilities|Array|MakeArray (Utilities|Struct|MakeControlRigComponentMappedComponent (Variables|Default|GetGuide_01) "point_1_ctrl" "Control" "Input") (Utilities|Struct|MakeControlRigComponentMappedComponent (Variables|Default|GetGuide_03) "point_3_ctrl" "Control" "Input") (Utilities|Struct|MakeControlRigComponentMappedComponent (Variables|Default|GetGuide_05) "point_5_ctrl" "Control" "Input") (Utilities|Struct|MakeControlRigComponentMappedComponent (Variables|Default|GetGuide_07) "point_7_ctrl" "Control" "Input"))))

(fn BPTornadoAutoGenFunc
  (params (Component :type Control%20Rig%20Component%20Object%20Reference))
  (Class|ControlRigComponent|AddMappedCompleteSkeletalMesh Component (Variables|Default|GetSKM_UPTornadoA))
  (Class|ControlRigComponent|AddMappedCompleteSkeletalMesh Component (Variables|Default|GetSKM_UPTornadoB))
  (Class|ControlRigComponent|AddMappedComponents Component (Utilities|Array|MakeArray (Utilities|Struct|MakeControlRigComponentMappedComponent (Variables|Default|GetGuide_07) "point_7_ctrl" "Control" "Input"))))