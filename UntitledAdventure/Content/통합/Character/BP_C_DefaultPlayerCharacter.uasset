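; Default player character that owns the inventory and handles item pickup, crafting results, attacking and UI windows.
; Bound events update the slot map Invens, stacking by item ID, deducting crafting materials and using the item DataTable type to place crafted items.
; The controller's attack event plays a shotgun montage and spawns an actor at AtkPoint, gated by Attacking.
; NumPad keys toggle inventory and equipment widgets, showing the cursor while either is open.
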(event Custom|커스텀이벤트
  (params (CraftItem_Map :type Map%20of%20Integers%20to%20Integers))
  ;[1 1 1] 인벤 생성과 제작과 줍기 이벤트 실행 (이동 필요)
  (CallFunction|인벤토리함수 CraftItem_Map))

(event Custom|Atk_Event_Hoon_이벤트
  ;[1 1 1] Attacking 모션
  (if (not (Variables|Default|GetAttacking))
    (Animation|Montage|PlayMontage (Variables|Character|GetMesh) "/Game/Hoon/Fire_Shotgun_Ironsights_Hoon_Montage.Fire_Shotgun_Ironsights_Hoon_Montage" 1.0 0.0 ""
      (:then
        (Variables|Default|SetAttacking true)
        (Default|CallAttackingEnventHoon (stale EventBeginPlay _astest_ct_hoon) true)
        (Game|SpawnActorfromClass "/Game/Hoon/Char_BluePrint/Spawn.Spawn_C" (Transformation|GetWorldTransform (Variables|Default|GetAtk_Point)) "Undefined" "MultiplyWithRoot" 0 0))
      (:OnCompleted
        (Variables|Default|SetAttacking false :!label _label)
        (Default|CallAttackingEnventHoon (stale EventBeginPlay _astest_ct_hoon) false))
      (:OnInterrupted
        (goto _label)))))

(event Custom|PickUp
  (params (ItemId :type Integer) (ItemCount :type Integer))
  ;[1 1 1] 인벤 생성과 제작과 줍기 이벤트 실행 (이동 필요)
  (CallFunction|PickUpItemF ItemId ItemCount))

(event Custom|커스텀이벤트_0
  (params (CraftItem_Num :type Integer) (ItemCount :type Integer))
  ;[1 1 1] 인벤 생성과 제작과 줍기 이벤트 실행 (이동 필요)
  (디폴트|인벤토리end함수 CraftItem_Num ItemCount))

(event Custom|인벤창%20이벤트
  (Default|InvenShow (Variables|Default|Get인벤블루프린트) (Variables|Default|GetInvens)))

(event Custom|장비창%20이벤트
  (Default|EquirShow (Variables|Default|Get장비블루프린트) (Variables|Default|GetEquirs)))

(event EventBeginPlay
  ;[1 1 1] 인벤 생성과 제작과 줍기 이벤트 실행 (이동 필요)
  (EventDispatchers|BindEventtoInventoryEvent (delegate Custom|커스텀이벤트))
  (EventDispatchers|BindEventtoInventoryEventEnd (delegate Custom|커스텀이벤트_0))
  (EventDispatchers|BindEventtoPickUpItem (delegate Custom|PickUp))
  ;[1 1 1] Attacking 모션
  (bind _astest_ct_hoon (Utilities|Casting|CastToTest_CT_Hoon (Pawn|GetController)))
  (EventDispatchers|AssignAtkEventHoon _astest_ct_hoon (delegate Custom|Atk_Event_Hoon_이벤트)))

(event Input|KeyboardEvents|NumPadThree
  (params (Key :type Key%20Structure :default "None"))
  (:Pressed
    (CallFunction|UIToggle "인벤")))

(event Input|KeyboardEvents|NumPadFour
  (params (Key :type Key%20Structure :default "None"))
  (:Pressed
    (CallFunction|UIToggle "장비")))

(fn ConstructionScript)

(fn PickUpItemF
  (params (ItemId :type Integer) (ItemCount :type Integer))
  (bind _invens (Variables|Default|GetInvens))
  (Development|PrintString (Utilities|String|Append (Utilities|String|ToString(Integer) ItemId) "번 아이템이" (Utilities|String|ToString(Integer) ItemCount) "증가한다."))
  (bind _values (Utilities|Map|Values _invens))
  (bind (_array_element _array_index) (Utilities|Array|ForEachLoopwithBreak _values :!label _label)
    (:LoopBody
      (if (== (.인덱스 _array_element) ItemId)
        (bind _output_get (LocalVariables|SetNewLocalVar (Utilities|Struct|MakeInvenItem_Structer_Hoon (.인덱스 _array_element) (+ (.겹친횟수 _array_element) ItemCount) (.현재내구도 _array_element))))
        (Utilities|Map|Add _invens _array_index _output_get)
        (bind _output_get_2 (LocalVariables|SetNewLocalVar_0 true))
        (Development|PrintString "주움")
        (goto _label Break)))
    (:Completed
      (if (not _output_get_2)
        (bind (_array_element_2 _array_index_2) (Utilities|Array|ForEachLoopwithBreak _values :!label _label_2)
          (:LoopBody
            (if (== (.인덱스 _array_element_2) 0)
              (bind _output_get_3 (LocalVariables|SetNewLocalVar (Utilities|Struct|MakeInvenItem_Structer_Hoon ItemId ItemCount 100)))
              (Utilities|Map|Add _invens _array_index_2 _output_get_3)
              (goto _label_2 Break))))))))

(fn 인벤토리함수
  (params (CraftItem_Map :type Map%20of%20Integers%20to%20Integers))
  (bind _values (Utilities|Map|Values CraftItem_Map))
  (bind _keys (Utilities|Map|Keys CraftItem_Map))
  (bind _values_2 (Utilities|Map|Values (Variables|Default|GetInvens)))
  (for (_array_element _array_index) _keys
    (bind (_array_element_2 _array_index_2) (Utilities|Array|ForEachLoopwithBreak _values_2 :!label _label)
      (:LoopBody
        (if (== _array_element (.인덱스 _array_element_2))
          (Utilities|Map|Add (Variables|Default|GetInvens) _array_index_2 (Utilities|Struct|MakeInvenItem_Structer_Hoon (.인덱스 _array_element_2) (- (.겹친횟수 _array_element_2) (Utilities|Array|Get(acopy) _values _array_index)) (.현재내구도 _array_element_2)))
          (goto _label Break))))))

(fn 인벤토리end함수
  (params (CraftItemNum :type Integer) (ItemCount :type Integer))
  (LocalVariables|SetCraftItem false)
  (Variables|Default|SetItemAdd false)
  (bind _values (Utilities|Map|Values (Variables|Default|GetInvens)))
  (bind _returnvalue (Utilities|GetDataTableRow "/Game/통합/Table/아이템Table.아이템Table" (Utilities|String|StringToName (Utilities|String|ToString(Integer) CraftItemNum)))
    (:then
      _)
    (:RowNotFound
      _))
  (if (Utilities|Enum|Equal(Enum) (.type _returnvalue) "NewEnumerator2")
    (bind (_array_element _array_index) (Utilities|Array|ForEachLoopwithBreak _values :!label _label)
      (:LoopBody
        (if (== (.인덱스 _array_element) 0)
          (Utilities|Map|Add (Variables|Default|GetInvens) _array_index (Utilities|Struct|MakeInvenItem_Structer_Hoon CraftItemNum ItemCount 100))
          (LocalVariables|SetCraftItem true)
          (goto _label Break)))
      (:Completed
        (if (not (LocalVariables|GetCraftItem))
          (Development|PrintString "인벤 자리가 부족합니다."))))
    (else
      (bind (_array_element_2 _array_index_2) (Utilities|Array|ForEachLoopwithBreak _values :!label _label_2)
        (:LoopBody
          (if (== (.인덱스 _array_element_2) CraftItemNum)
            (Utilities|Map|Add (Variables|Default|GetInvens) _array_index_2 (Utilities|Struct|MakeInvenItem_Structer_Hoon (.인덱스 _array_element_2) (+ (.겹친횟수 _array_element_2) ItemCount) (.현재내구도 _array_element_2)))
            (bind _output_get (Variables|Default|SetItemAdd true))
            (goto _label_2 Break)))
        (:Completed
          (if (not _output_get)
            (goto _label)))))))

(fn UIToggle
  (params (windowName :type String))
  (bind _returnvalue (Game|GetPlayerController 0))
  (bind _output_get (LocalVariables|SetWindowNames windowName))
  (if (.Value (Utilities|Map|Find (Variables|Default|GetNameAndBool) _output_get))
    (switch string (LocalVariables|GetWindowNames)
      (:인벤
        (Widget|RemovefromParent (Variables|Default|Get인벤블루프린트))
        (Variables|Default|Set인벤블루프린트 0))
      (:장비
        (Widget|RemovefromParent (Variables|Default|Get장비블루프린트))
        (Variables|Default|Set장비블루프린트 0)))
    (Utilities|Map|Add (Variables|Default|GetNameAndBool) (LocalVariables|GetWindowNames) false)
    (else
      (switch string (LocalVariables|GetWindowNames)
        (:인벤
          (bind _returnvalue_2 (UserInterface|CreateWidget (LocalVariables|Get인벤클래스)))
          (UserInterface|Viewport|AddtoViewport _returnvalue_2 0)
          (Variables|Default|Set인벤블루프린트 _returnvalue_2)
          (CallFunction|인벤창이벤트))
        (:장비
          (bind _returnvalue_3 (UserInterface|CreateWidget (LocalVariables|Get장비클래스)))
          (UserInterface|Viewport|AddtoViewport _returnvalue_3 0)
          (Variables|Default|Set장비블루프린트 _returnvalue_3)
          (CallFunction|장비창이벤트)))
      (Utilities|Map|Add (Variables|Default|GetNameAndBool) (LocalVariables|GetWindowNames) true)))
  (bind _values (Utilities|Map|Values (Variables|Default|GetNameAndBool)))
  (bind _array_element (Utilities|Array|ForEachLoopwithBreak _values :!label _label)
    (:LoopBody
      (if _array_element
        (Variables|/Script/Engine.PlayerController|SetbShowMouseCursor _returnvalue true)
        (goto _label Break)
        (else
          (Variables|/Script/Engine.PlayerController|SetbShowMouseCursor _returnvalue false))))))