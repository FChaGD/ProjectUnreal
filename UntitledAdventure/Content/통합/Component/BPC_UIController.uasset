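; BPC_UIController is a component that shows and removes dialogue script and NPC choice widgets.
; ShowScript lazily creates the dialogue widget, sets caster and name, then types the text one character at a time via re-armed, randomly delayed timers.
; ShowSelect lazily creates the choice widget, fills it and flags the player controller as selecting.
; FinishTheTyping overwrites the displayed string; GetIsTyping always returns false, ignoring the Istyping flag.
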(event Custom|Show%20Script
  (params (Name :type String) (Script :type String) (Caster :type Actor%20Object%20Reference))
  ;[1 1 1] 스크립트 출력
  (Variables|Default|SetDisplayScrpit "")
  (|Typing_2 Name Script Caster))

(event Custom|Finish%20The%20Typing
  (params (Script :type String))
  ;[1 1 1] 스크립트 출력
  (Variables|Default|SetDisplayScrpit Script))

(event Custom|Show%20Select
  (params (Caster :type Actor%20Object%20Reference) (Data :type Array%20of%20ST%20Select%20Data%20Structures))
  ;[1 1 1] 선택지 출력
  (Utilities|IsValid (Variables|Default|GetNPCSelect)
    (:Is%20Valid
      _)
    (:Is%20Not%20Valid
      ;;[1 1 1] ui 생성
      (bind _returnvalue (UserInterface|CreateWidget "/Game/통합/UI/NPCUI/BP_NPCSelect.BP_NPCSelect_C" (Game|GetPlayerController 0)))
      (bind _output_get (Variables|Default|SetNPCSelect _returnvalue))))
  (Default|SetCaster (Variables|Default|GetNPCSelect) Caster)
  (Default|SetDataList (Variables|Default|GetNPCSelect) Data)
  (Default|MakeSelect (Variables|Default|GetNPCSelect))
  (UserInterface|Viewport|AddtoViewport _output_get 0)
  (Class|BPATIControllerInterface|IsSelecting(Message) (Game|GetPlayerController 0) true))

(event Custom|Clean%20Select
  (bind _npcselect (Variables|Default|GetNPCSelect))
  ;[1 1 1] 선택지 제거
  (Utilities|IsValid _npcselect
    (:Is%20Valid
      (Default|ClearSelect _npcselect)
      (Widget|RemovefromParent _npcselect))))

(event Custom|Clean%20Scirpt
  (bind _scriptwidget (Variables|Default|GetScriptWidget))
  ;[1 1 1] 스크립트 ui 제거
  (Utilities|IsValid _scriptwidget
    (:Is%20Valid
      (Widget|RemovefromParent _scriptwidget))))

(event EventBeginPlay)

(event EventTick
  (params (DeltaSeconds :type Float%20%28single-precision%29)))

(event EventShowSelect
  (params (Caster :type %20Object%20Reference))
  ;[1 1 1] 선택지 출력
)

(event Custom|RepeatTyping
  ;[1 1 1] UISetting
  (bind _returnvalue (Utilities|Time|SetTimerbyEvent (EventDispatchers|CreateEvent :!event Custom|TypeWriting) (Math|Random|RandomFloatinRange 0.02 0.07)))
  (Variables|Default|SettypeWriterTimer _returnvalue))

(event Custom|TypeWriting
  (Utilities|FlowControl|Sequence
    (:then_0
      ;[1 1 1] 스크립트 분할
      (Variables|Default|SetDisplayScrpit (Utilities|String|GetSubstring (stale _scrpit) 0 (+ (Utilities|String|Len (Variables|Default|GetDisplayScrpit)) 1))))
    (:then_1
      ;[1 1 1] UI 스크립트 출력
      (Default|SetContent (Variables|Default|GetScriptWidget) (Variables|Default|GetDisplayScrpit)))
    (:then_2
      ;[1 1 1] looping
      (if (Utilities|Enum|Equal(Enum) (stale _scrpit) (Variables|Default|GetDisplayScrpit))
        ;[1 1 1] 타이핑 종료
        (Utilities|Time|ClearandInvalidateTimerbyHandle (Variables|Default|GettypeWriterTimer))
        (Variables|Default|SetIstyping? false)
        (return)
        (else
          (CallFunction|RepeatTyping))))))

(fn GetIsTyping?
  (return false))