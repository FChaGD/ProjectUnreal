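; Player skill system that tracks unlocked skill tiers in the SkillUnlocks map and implements the skill actions.
; 염원의화 spawns a fireball at the player's SkillArrow.
; 한기의탄 fires ice bullets at entries in Targets, which gains enemies within range up to four and is never cleared here.
; 뒤바람의순리 performs a boosted jump, stronger while running, with buff particles and clears IsAbleToSkill3; 화극금 and 수생목 are empty stubs.
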(event EventBeginPlay)

(event EventTick
  (params (DeltaSeconds :type Float%20%28single-precision%29)))

(fn AddSkill
  (params (Row_Name :type String))
  (bind _skillunlocks (Variables|Default|GetSkillUnlocks))
  (bind (_value _returnvalue) (Utilities|Map|Find _skillunlocks Row_Name))
  (if _returnvalue
    (Utilities|Map|Add (Variables|Default|GetSkillUnlocks) Row_Name (+ _value 1))
    (return true)
    (else
      (Utilities|Map|Add (Variables|Default|GetSkillUnlocks) Row_Name 1)
      (return true))))

(fn QuerySkill
  (params (Row_Name :type String))
  (bind _skillunlocks (Variables|Default|GetSkillUnlocks))
  (bind (_value _returnvalue) (Utilities|Map|Find _skillunlocks Row_Name))
  (if _returnvalue
    (return true _value)
    (else
      (return false 0))))

(fn 염원의화
  (bind _asbp_c_default_player_character (Utilities|Casting|CastToBP_C_DefaultPlayerCharacter (Game|GetPlayerCharacter 0)))
  (Game|SpawnActorfromClass "/Game/SeoK/Object/BP_FIreBall.BP_FIreBall_C" (Transformation|GetWorldTransform (Variables|/Game/통합/Character/BP_C_DefaultPlayerCharacter.BP_C_DefaultPlayerCharacter_C|GetSkill%20Arrow _asbp_c_default_player_character)) "Undefined" "MultiplyWithRoot" 0 0))

(fn 한기의탄
  (bind _targets (Variables|Default|GetTargets))
  (bind _asbp_c_default_player_character (Utilities|Casting|CastToBP_C_DefaultPlayerCharacter (Game|GetPlayerCharacter 0)))
  (bind _outactors (Actor|GetAllActorsOfClass "/Game/통합/Monster/BP_EnemyAI.BP_EnemyAI_C"))
  (for _array_element _outactors
    (if (<= (Transformation|GetDistanceTo (Game|GetPlayerCharacter 0) _array_element) 8e+02)
      (if (<= (Utilities|Array|Length _targets) 3)
        (Utilities|Array|Add _targets _array_element))))
  (for _array_element_2 (Variables|Default|GetTargets)
    (bind _returnvalue (Game|SpawnActorfromClass "/Game/SeoK/Object/BP_iceBullet.BP_iceBullet_C" (Transformation|GetWorldTransform (Variables|/Game/통합/Character/BP_C_DefaultPlayerCharacter.BP_C_DefaultPlayerCharacter_C|GetSkill%20Arrow _asbp_c_default_player_character)) "Undefined" "MultiplyWithRoot" 0 0))
    (Default|Init _returnvalue _array_element_2 (.Location (Math|Transform|BreakTransform (Transformation|GetWorldTransform (Variables|/Game/통합/Character/BP_C_DefaultPlayerCharacter.BP_C_DefaultPlayerCharacter_C|GetSkill%20Arrow _asbp_c_default_player_character)))))))

(fn 뒤바람의순리
  (bind _aspc_default_pc (Utilities|Casting|CastToPC_DefaultPC (Game|GetPlayerController 0)))
  (if (Variables|/Game/통합/Map/PC_DefaultPC.PC_DefaultPC_C|GetRunning _aspc_default_pc)
    (Variables|/Script/Engine.CharacterMovementComponent|SetJumpZVelocity (Variables|/Game/통합/Map/PC_DefaultPC.PC_DefaultPC_C|GetCharacter%20Movement _aspc_default_pc) (* (+ (Variables|/Game/통합/Map/PC_DefaultPC.PC_DefaultPC_C|GetJumpUP _aspc_default_pc) 2e+02) 1.5))
    (Variables|Default|SetIs%20Able%20to%20Skill3 false)
    (bind _asbp_c_default_player_character (Utilities|Casting|CastToBP_C_DefaultPlayerCharacter (Game|GetPlayerCharacter 0)))
    (Character|Jump _asbp_c_default_player_character)
    (Components|Activation|Activate (Variables|/Game/통합/Character/BP_C_DefaultPlayerCharacter.BP_C_DefaultPlayerCharacter_C|GetBuffParticle _asbp_c_default_player_character) false)
    (else
      (Variables|/Script/Engine.CharacterMovementComponent|SetJumpZVelocity (Variables|/Game/통합/Map/PC_DefaultPC.PC_DefaultPC_C|GetCharacter%20Movement _aspc_default_pc) (* (Variables|/Game/통합/Map/PC_DefaultPC.PC_DefaultPC_C|GetJumpUP _aspc_default_pc) 1.5))
      (Variables|Default|SetIs%20Able%20to%20Skill3 false)
      (bind _asbp_c_default_player_character_2 (Utilities|Casting|CastToBP_C_DefaultPlayerCharacter (Game|GetPlayerCharacter 0)))
      (Character|Jump _asbp_c_default_player_character_2)
      (Components|Activation|Activate (Variables|/Game/통합/Character/BP_C_DefaultPlayerCharacter.BP_C_DefaultPlayerCharacter_C|GetBuffParticle _asbp_c_default_player_character_2) false))))

(fn 화극금)

(fn 수생목)