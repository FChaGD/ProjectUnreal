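; Base Blueprint for NPC interaction, driving dialogue, answer selection, speech bubbles and merchant UI.
; Interaction switches on the current type, starting from DefaultInteraction, and resolves content through link-table lookups.
; Text and choices display through the GameMode's BPC_UIController, with SelectAnswer jumping into the next type's branch.
; Merchants open craft or shop widgets, while input mode, cursor and controller hold toggle around interactions.
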(event Custom|CustomEvent
  (params (InteractionId :type Integer))
  (bind _outrownames (DataTable|GetDataTableRowNames "/Game/통합/Table/BP_DT_EndSequence.BP_DT_EndSequence"))
  (for _array_element _outrownames
    (bind _returnvalue (Utilities|GetDataTableRow "/Game/통합/Table/BP_DT_EndSequence.BP_DT_EndSequence" _array_element)
      (:then
        (if (== InteractionId (.InteractionId (Utilities|Struct|BreakTS_EndSequence _returnvalue)))
          (switch Utilities|FlowControl|Switch|SwitchonEN_EndSequence (.EndSequence (Utilities|Struct|BreakTS_EndSequence _returnvalue))))))))

(event Custom|CustomEvent_1
  (bind _returnvalue (Game|GetPlayerController 0))
  ;[1 1 1] 상호작용 종료
  (Default|CleanScirpt (Variables|Default|GetUI%20Controller))
  (Variables|Default|SetCurrentInteraction "NewEnumerator3")
  (Input|SetInputModeGameOnly _returnvalue false)
  (Variables|/Script/Engine.PlayerController|SetbShowMouseCursor _returnvalue false)
  (Class|BPATIControllerInterface|ControllerHoldSet(Message) (Game|GetPlayerController 0) true))

(event Custom|CustomEvent_3
  (bind _returnvalue (Game|GetPlayerController 0))
  (Variables|Default|SetCraftUI 0)
  (Variables|Default|SetShopUI 0)
  ;[1 1 1] 상호작용 종료
  (Default|CleanScirpt (Variables|Default|GetUI%20Controller))
  (Variables|Default|SetCurrentInteraction "NewEnumerator3")
  (Input|SetInputModeGameOnly _returnvalue false)
  (Variables|/Script/Engine.PlayerController|SetbShowMouseCursor _returnvalue false)
  (Class|BPATIControllerInterface|ControllerHoldSet(Message) (Game|GetPlayerController 0) true))

(event Collision|EventActorBeginOverlap
  (params (OtherActor :type Actor%20Object%20Reference)))

(event EventTick
  (params (DeltaSeconds :type Float%20%28single-precision%29)))

(event EventSelectAnswer
  (params (Selection :type Integer) (nextInteractionType :type EN_InteractionType%20Enum :default "NewEnumerator1"))
  (Variables|Default|SetPreScriptId (Variables|Default|GetScriptId))
  (Variables|Default|SetScriptId Selection)
  (Class|BPATIControllerInterface|IsSelecting(Message) (Game|GetPlayerController 0) false)
  (switch Utilities|FlowControl|Switch|SwitchonEN_InteractionType nextInteractionType
    (:NewEnumerator1
      ;[1 1 1] 대화
      (Default|CleanSelect (Variables|Default|GetUI%20Controller))
      (Variables|Default|SetCurrentInteraction "NewEnumerator1")
      (if (Variables|Default|GetIsScriptOver)
        _
        (else
          (bind _interactionidtarget (CallFunction|FindLinkTableRow "NewEnumerator1"))
          (Variables|Default|SetIsScriptOver true)))
      (bind (_endsequence _countinue) (CallFunction|ScriptGenerate _interactionidtarget))
      (if _countinue
        (CallFunction|InteractingEndSequnce _endsequence)))
    (:NewEnumerator4
      (if (Variables|/Game/통합/Component/BPC_UIController.BPC_UIController_C|GetIstyping? (Variables|Default|GetUI%20Controller))
        ;[1 1 1] 선택지 전 스크립트 출력 예외처리
        (bind _returnvalue (Utilities|GetDataTableRow (Variables|Default|GetScriptTable) (Utilities|String|StringToName (Utilities|String|ToString(Integer) (Variables|Default|GetPreScriptId))))
          (:then
            (Default|FinishtheTyping (Variables|Default|GetUI%20Controller) (.Script (Utilities|Struct|BreakTS_Script _returnvalue)))))
        (else
          ;[1 1 1] 선택지 상호작용
          (Default|CleanScirpt (Variables|Default|GetUI%20Controller))
          (bind _selectlist (CallFunction|SelectList (Variables|Default|GetScriptId)))
          (Default|ShowSelect (Variables|Default|GetUI%20Controller) self _selectlist)
          (Variables|Default|SetScriptId 0)
          (CallFunction|InteractingEndSequnce (Variables|Default|GetPreScriptId))
          (Variables|Default|SetPreScriptId 0))))
    (:NewEnumerator6
      ;[1 1 1] 상호작용
      (Variables|Default|SetCurrentInteraction "NewEnumerator6")
      (if (Variables|Default|GetIsScriptOver)
        _
        (else
          (bind _interactionidtarget_2 (CallFunction|FindLinkTableRow "NewEnumerator6"))
          (Variables|Default|SetIsScriptOver true)))
      (bind _endsequence_2 (CallFunction|GenerateBubble _interactionidtarget_2))
      (CallFunction|InteractingEndSequnce _endsequence_2))))

(event EventInteraction
  (bind _returnvalue (Game|GetPlayerController 0))
  (bind _returnvalue_2 (Game|GetPlayerController 0))
  (bind _self self)
  (if (and (Utilities|Enum|Equal(Enum) (Variables|Default|GetCurrentInteraction) "NewEnumerator3") (Utilities|Enum|Equal(Enum) "NewEnumerator6" (Variables|Default|GetDefaultInteraction)))
    _
    (elif (and (Utilities|Enum|NotEqual(Enum) (Variables|Default|GetCurrentInteraction) "NewEnumerator3") (Utilities|Enum|Equal(Enum) "NewEnumerator6" (Variables|Default|GetDefaultInteraction)))
      ;[1 1 1] 말풍선 상호작용 관련 inputmode & mouse cursor
      (Class|BPATIControllerInterface|ControllerHoldSet(Message) _returnvalue false)
      (Input|SetInputModeGameandUI _returnvalue 0 "DoNotLock" true false)
      (Variables|/Script/Engine.PlayerController|SetbShowMouseCursor _returnvalue true)
      (else
        (Class|BPATIControllerInterface|ControllerHoldSet(Message) (Game|GetPlayerController 0) false))))
  (switch Utilities|FlowControl|Switch|SwitchonEN_InteractionType (Variables|Default|GetCurrentInteraction) :!label _label
    (:NewEnumerator1
      ;[1 1 1] 대화
      (Default|CleanSelect (Variables|Default|GetUI%20Controller))
      (Variables|Default|SetCurrentInteraction "NewEnumerator1")
      (if (Variables|Default|GetIsScriptOver)
        _
        (else
          (bind _interactionidtarget (CallFunction|FindLinkTableRow "NewEnumerator1"))
          (Variables|Default|SetIsScriptOver true)))
      (bind (_endsequence _countinue) (CallFunction|ScriptGenerate _interactionidtarget))
      (if _countinue
        (CallFunction|InteractingEndSequnce _endsequence)))
    (:NewEnumerator4
      (if (Variables|/Game/통합/Component/BPC_UIController.BPC_UIController_C|GetIstyping? (Variables|Default|GetUI%20Controller))
        ;[1 1 1] 선택지 전 스크립트 출력 예외처리
        (bind _returnvalue_3 (Utilities|GetDataTableRow (Variables|Default|GetScriptTable) (Utilities|String|StringToName (Utilities|String|ToString(Integer) (Variables|Default|GetPreScriptId))))
          (:then
            (Default|FinishtheTyping (Variables|Default|GetUI%20Controller) (.Script (Utilities|Struct|BreakTS_Script _returnvalue_3)))))
        (else
          ;[1 1 1] 선택지 상호작용
          (Default|CleanScirpt (Variables|Default|GetUI%20Controller))
          (bind _selectlist (CallFunction|SelectList (Variables|Default|GetScriptId)))
          (Default|ShowSelect (Variables|Default|GetUI%20Controller) self _selectlist)
          (Variables|Default|SetScriptId 0)
          (CallFunction|InteractingEndSequnce (Variables|Default|GetPreScriptId))
          (Variables|Default|SetPreScriptId 0))))
    (:NewEnumerator5
      (Development|PrintString "상인 접근")
      ;[1 1 1] 상인/ npc id와 InteractionId로 원하는 상인으로 이동해야함
      (Variables|Default|SetCurrentInteraction "NewEnumerator5")
      (bind _interactionidtarget_2 (CallFunction|FindLinkTableRow "NewEnumerator5"))
      (switch int _interactionidtarget_2
        (:0
          (if (not (Utilities|IsValid (Variables|Default|GetCraftUI)))
            (bind _returnvalue_4 (UserInterface|CreateWidget "/Game/통합/UI/CraftUI/Tool_WidgetBlueprint_Hoon.Tool_WidgetBlueprint_Hoon_C"))
            (bind _output_get (Variables|Default|SetCraftUI _returnvalue_4))
            (Default|GetNpc _output_get _self)
            (UserInterface|Viewport|AddtoViewport _output_get 0)))
        (:1
          (if (not (Utilities|IsValid (Variables|Default|GetShopUI)))
            (bind _returnvalue_5 (UserInterface|CreateWidget "/Game/Hoon/연습/ShopBP_Hoon.ShopBP_Hoon_C"))
            (bind _output_get_2 (Variables|Default|SetShopUI _returnvalue_5))
            (Default|GetNPC _output_get_2 _self)
            (UserInterface|Viewport|AddtoViewport _output_get_2 0)))))
    (:NewEnumerator6
      ;[1 1 1] 상호작용
      (Variables|Default|SetCurrentInteraction "NewEnumerator6")
      (if (Variables|Default|GetIsScriptOver)
        _
        (else
          (bind _interactionidtarget_3 (CallFunction|FindLinkTableRow "NewEnumerator6"))
          (Variables|Default|SetIsScriptOver true)))
      (bind _endsequence_2 (CallFunction|GenerateBubble _interactionidtarget_3))
      (CallFunction|InteractingEndSequnce _endsequence_2))
    (:NewEnumerator3
      (if (== (Variables|Default|GetScriptId) -1)
        (Variables|Default|SetPreScriptId 0)
        (Variables|Default|SetScriptId 0)
        (CallFunction|EndInteraction)
        (else
          ;[1 1 1] 대화 종류가 아무것도 없을 경우
          (Variables|Default|SetUI%20Controller (Actor|GetComponentbyClass (Game|GetGameMode) "/Game/통합/Component/BPC_UIController.BPC_UIController_C"))
          (bind _output_get_3 (Variables|Default|SetCurrentInteraction (Variables|Default|GetDefaultInteraction)))
          (if (Utilities|Enum|Equal(Enum) _output_get_3 "NewEnumerator6")
            (goto _label)
            (else
              (Input|SetInputModeGameandUI _returnvalue_2 0 "DoNotLock" true false)
              (Variables|/Script/Engine.PlayerController|SetbShowMouseCursor _returnvalue_2 true)
              (goto _label))))))))

(fn ConstructionScript
  (|CallParentFunction))